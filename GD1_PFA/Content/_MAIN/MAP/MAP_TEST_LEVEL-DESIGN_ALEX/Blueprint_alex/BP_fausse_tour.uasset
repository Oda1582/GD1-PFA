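; BP_fausse_tour is a sweeping surveillance camera ("fausse tour") with a cone mesh, in a level-design test map folder.
; A timeline yaws the root back and forth across a configurable angle centred on the yaw stored at construction.
; When each sweep finishes, it pauses, then a FlipFlop alternates reverse and forward playback.
; The construction script applies the rotation speed and cone scale.
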(event Custom|update_cam
  (bind _degré_de_rotation (Variables|Paramètrescaméra|Getdegré%20de%20rotation))
  ;[1 1 1 1 45] Fait tourner la caméra
  (Utilities|FlowControl|FlipFlop
    (:A
      (bind _rotation (Timeline|animation%20de%20rotation ReverseFromEnd)
        (:Update
          (Transformation|SetRelativeRotation (Variables|Default|GetDefaultSceneRoot) (Math|Rotator|MakeRotator 0.0 0.0 (+ (Variables|Default|Getposition%20d'origine) (- (* _rotation _degré_de_rotation) (/ _degré_de_rotation 2)))) false false))
        (:Finished
          (Utilities|FlowControl|Delay (Variables|ParamètresCaméra|Getpause%20%28en%20secondes%29))
          (CallFunction|UpdateCam))))
    (:B
      (Timeline|animation%20de%20rotation PlayFromStart))))

(event EventBeginPlay
  (bind _degré_de_rotation (Variables|Paramètrescaméra|Getdegré%20de%20rotation))
  ;[1 1 1 1 45] Fait tourner la caméra
  (bind _rotation (Timeline|animation%20de%20rotation PlayFromStart)
    (:Update
      (Transformation|SetRelativeRotation (Variables|Default|GetDefaultSceneRoot) (Math|Rotator|MakeRotator 0.0 0.0 (+ (Variables|Default|Getposition%20d'origine) (- (* _rotation _degré_de_rotation) (/ _degré_de_rotation 2)))) false false))
    (:Finished
      (Utilities|FlowControl|Delay (Variables|ParamètresCaméra|Getpause%20%28en%20secondes%29))
      (CallFunction|UpdateCam))))

(fn ConstructionScript
  (bind _longueur_conne (Variables|ParamètresCaméra|Getlongueur%20conne))
  (Utilities|FlowControl|Sequence
    (:then_0
      ;[1 1 1] permet de changer la vitesse de l'animation de rotation des caméras en changant la valeur de " vitesse rotation "
      (Components|Timeline|SetPlayRate (Variables|Default|Getanimation%20de%20rotation) (Variables|Paramètrescaméra|Getvitesse%20de%20rotation)))
    (:then_1
      ;[1 1 1] Change la porté du cone
      (Transformation|SetRelativeScale3D (Variables|Default|GetSM_fausse_tour_cone) (Math|Vector|MakeVectorNetQuantize _longueur_conne _longueur_conne _longueur_conne)))
    (:then_2
      ;[1 1 1] Permet de stocker la position de la caméra
      (Variables|Default|Setposition%20d'origine (.yaw (Transformation|GetActorRotation))))))