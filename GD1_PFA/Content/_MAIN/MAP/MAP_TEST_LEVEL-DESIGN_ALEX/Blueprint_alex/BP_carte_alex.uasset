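; BP_carte_alex is a keycard pickup that comes in green, yellow or red.
; The construction script tints a dynamic instance of M_carte_alex according to the NuméroCarte type.
; When BP_FirstPersonCharacter overlaps it, it calls NiveauSup on every BP_grille_lente in the level, then destroys itself.
; The card type only affects the color, and the GM_Game reference cached on BeginPlay is unused here.
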(event OnComponentBeginOverlap(carte_clé)
  (params (OverlappedComponent :type Primitive%20Component%20Object%20Reference) (OtherActor :type Actor%20Object%20Reference) (OtherComp :type Primitive%20Component%20Object%20Reference) (OtherBodyIndex :type Integer) (bFromSweep :type Boolean) (SweepResult :type Hit%20Result%20Structure%20%28by%20ref%29))
  (Utilities|Casting|CastToBP_FirstPersonCharacter OtherActor)
  (bind _outactors (Actor|GetAllActorsOfClass "/Game/_MAIN/MAP/MAP_TEST_LEVEL-DESIGN_ALEX/Blueprint_alex/BP_grille_lente.BP_grille_lente_C"))
  (Default|NiveauSup _outactors)
  (Actor|DestroyActor))

(event EventBeginPlay
  (bind _asgm_game (Utilities|Casting|CastToGM_Game (Game|GetGameMode)))
  (Variables|Default|SetGM _asgm_game))

(fn ConstructionScript
  (bind _nom_paramètre_m (Variables|Default|Getnom_paramètre_M))
  ;[1 1 1] Change l'affichage selon le type de clé
  (bind _returnvalue (Rendering|Material|CreateDynamicMaterialInstance (Variables|Default|Getcarte%20_clé) 0 "/Game/_MAIN/MAP/MAP_TEST_LEVEL-DESIGN_ALEX/Matérials/M_carte_alex.M_carte_alex" "None" :!class /Script/Engine.PrimitiveComponent))
  (switch Utilities|FlowControl|Switch|Switchonenum_carte_alex (Variables|Default|Getnuméro%20carte)
    (:NewEnumerator0
      (Rendering|Material|SetVectorParameterValue _returnvalue _nom_paramètre_m "(R=0.000000,G=0.750000,B=0.040244,A=1.000000)" :!class /Script/Engine.MaterialInstanceDynamic))
    (:NewEnumerator1
      (Rendering|Material|SetVectorParameterValue _returnvalue _nom_paramètre_m "(R=0.986004,G=1.000000,B=0.000000,A=1.000000)" :!class /Script/Engine.MaterialInstanceDynamic))
    (:NewEnumerator2
      (Rendering|Material|SetVectorParameterValue _returnvalue _nom_paramètre_m "(R=1.000000,G=0.016558,B=0.000000,A=1.000000)" :!class /Script/Engine.MaterialInstanceDynamic))))