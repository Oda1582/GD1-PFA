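; Slow grate actor that rises when the player overlaps its box, waits, then lowers itself.
; A FlipFlop alternates the two MoveComponentTo animations, with the AnimFini flag blocking retriggers until each finishes.
; The Selection enum (blue, yellow, red) sets timings and dynamic material color.
; NiveauSup counts obtained keys to switch the grate to yellow or red, shortening its open window and slowing its rise.
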(event OnComponentBeginOverlap(Box)
  (params (OverlappedComponent :type Primitive%20Component%20Object%20Reference) (OtherActor :type Actor%20Object%20Reference) (OtherComp :type Primitive%20Component%20Object%20Reference) (OtherBodyIndex :type Integer) (bFromSweep :type Boolean) (SweepResult :type Hit%20Result%20Structure%20%28by%20ref%29))
  (bind _grille (Variables|Default|Getgrille))
  ;[0.4688 0 0 1 45] Système de grille qui prend du temps à remonter
  ;;[1 1 1] Vérifie que c'est le joueur
  (Utilities|Casting|CastToBP_FirstPersonCharacter OtherActor)
  ;;[1 1 1] Vérifie que y'a pas déjà une des animations qu'est lancé
  (if (Variables|Default|GetAnim_fini)
    ;;[1 1 1] Permet de lancer ll'autre animation
    (Utilities|FlowControl|FlipFlop
      (:A
        ;;[1 1 1] Dis qu'une des animations se lance
        (Variables|Default|SetAnim_fini false)
        ;;[1 1 1] Fait monter / descendre la grille
        (Components|MoveComponentTo _grille "0, 0,140.000000" "0, 0, 0" false false (Variables|OPTIONDALLES|Gettemps%20monté) false)
        ;;[1 1 1] Indique que l'animation est fini
        (Variables|Default|SetAnim_fini true)
        ;;[1 1 1] Temps avant que la grille ne rebaisse
        (Utilities|FlowControl|Delay (Variables|OPTIONDALLES|Gettemps%20avant%20rebaisse))
        ;;[1 1 1] Execute l'animation de baisse
        (CallFunction|FermerGrille))
      (:B
        (Variables|Default|SetAnim_fini false)
        (Components|MoveComponentTo _grille "0, 0, 0" "0, 0, 0" false false (Variables|OPTIONDALLES|Gettemps%20descente) false)
        (Utilities|FlowControl|Delay (Variables|OPTIONDALLES|Gettemps%20end-lag))
        (Variables|Default|SetAnim_fini true)))))

(event Custom|fermer%20grille
  (bind _grille (Variables|Default|Getgrille))
  ;[0.4688 0 0 1 45] Système de grille qui prend du temps à remonter
  ;;[1 1 1] Vérifie que y'a pas déjà une des animations qu'est lancé
  (if (Variables|Default|GetAnim_fini)
    ;;[1 1 1] Permet de lancer ll'autre animation
    (Utilities|FlowControl|FlipFlop
      (:A
        ;;[1 1 1] Dis qu'une des animations se lance
        (Variables|Default|SetAnim_fini false)
        ;;[1 1 1] Fait monter / descendre la grille
        (Components|MoveComponentTo _grille "0, 0,140.000000" "0, 0, 0" false false (Variables|OPTIONDALLES|Gettemps%20monté) false)
        ;;[1 1 1] Indique que l'animation est fini
        (Variables|Default|SetAnim_fini true)
        ;;[1 1 1] Temps avant que la grille ne rebaisse
        (Utilities|FlowControl|Delay (Variables|OPTIONDALLES|Gettemps%20avant%20rebaisse))
        ;;[1 1 1] Execute l'animation de baisse
        (CallFunction|FermerGrille))
      (:B
        (Variables|Default|SetAnim_fini false)
        (Components|MoveComponentTo _grille "0, 0, 0" "0, 0, 0" false false (Variables|OPTIONDALLES|Gettemps%20descente) false)
        (Utilities|FlowControl|Delay (Variables|OPTIONDALLES|Gettemps%20end-lag))
        (Variables|Default|SetAnim_fini true)))))

(event Custom|niveau%20sup
  ;[1 1 1 1 45] Récupère depuis le GM le niveau des dalles
  (Variables|Default|Setnombre%20clés%20obtenus (+ 1 (Variables|Default|Getnombre%20clés%20obtenus)))
  (switch int (Variables|Default|Getnombre%20clés%20obtenus)
    (:0
      (Variables|Default|SetSelection "NewEnumerator1")
      (CallFunction|UpdateVitesse :!label _label))
    (:1
      (Variables|Default|SetSelection "NewEnumerator2")
      (goto _label))
    (:2
      (Development|PrintString "Niveau max"))))

(event Custom|update_vitesse
  ;[1 1 1 1 45] Adapte le type de dalle à la progression du joueur
  (Utilities|FlowControl|Sequence
    (:then_0
      ;[0 1 0.02065 1 45] Gère les durées
      (switch Utilities|FlowControl|Switch|Switchonenum_grille_lente (Variables|Default|GetSelection)
        (:NewEnumerator0
          ;;[1 1 1] Gère le temps que la grille met à monté
          (Variables|OPTIONDALLES|Settemps%20monté 1.5)
          ;;[1 1 1] Gère le temps que la grille met à descendre
          (Variables|OPTIONDALLES|Settemps%20descente 3.5)
          ;;[1 1 1] Gère le temps avant que la grille ne retombe
          (Variables|OPTIONDALLES|Settemps%20avant%20rebaisse 5.0)
          ;;[1 1 1] Gère le temps pendant le quelle la grille n'est pas utilisable
          (Variables|OPTIONDALLES|Settemps%20end-lag 0.0))
        (:NewEnumerator1
          (Variables|OPTIONDALLES|Settemps%20monté 2.5)
          (Variables|OPTIONDALLES|Settemps%20descente 2.0)
          (Variables|OPTIONDALLES|Settemps%20avant%20rebaisse 1.0)
          (Variables|OPTIONDALLES|Settemps%20end-lag 1.0))
        (:NewEnumerator2
          (Variables|OPTIONDALLES|Settemps%20monté 5.0)
          (Variables|OPTIONDALLES|Settemps%20descente 1.0)
          (Variables|OPTIONDALLES|Settemps%20avant%20rebaisse 0.5)
          (Variables|OPTIONDALLES|Settemps%20end-lag 3.0))))
    (:then_1
      ;[1 1 1 1 45] Gère la couleur de la dalle
      (bind _returnvalue (Rendering|Material|CreateDynamicMaterialInstance (Variables|Default|Getgrille) 0 "/Game/_MAIN/MAP/MAP_TEST_LEVEL-DESIGN_ALEX/Matérials/M_grille_lente.M_grille_lente" "None" :!class /Script/Engine.PrimitiveComponent))
      (switch Utilities|FlowControl|Switch|Switchonenum_grille_lente (Variables|Default|GetSelection)
        (:NewEnumerator0
          (Rendering|Material|SetVectorParameterValue _returnvalue "couleur_rouge" "(R=0.000000,G=0.354708,B=1.000000,A=1.000000)" :!class /Script/Engine.MaterialInstanceDynamic))
        (:NewEnumerator1
          (Rendering|Material|SetVectorParameterValue _returnvalue "couleur_rouge" "(R=0.986004,G=1.000000,B=0.000000,A=1.000000)" :!class /Script/Engine.MaterialInstanceDynamic))
        (:NewEnumerator2
          (Rendering|Material|SetVectorParameterValue _returnvalue "couleur_rouge" "(R=1.000000,G=0.016558,B=0.000000,A=1.000000)" :!class /Script/Engine.MaterialInstanceDynamic))))))

(event EventBeginPlay
  ;[0 1 0.02065 1 45] Gère les durées
  (switch Utilities|FlowControl|Switch|Switchonenum_grille_lente (Variables|Default|GetSelection)
    (:NewEnumerator0
      ;;[1 1 1] Gère le temps que la grille met à monté
      (Variables|OPTIONDALLES|Settemps%20monté 1.5)
      ;;[1 1 1] Gère le temps que la grille met à descendre
      (Variables|OPTIONDALLES|Settemps%20descente 3.5)
      ;;[1 1 1] Gère le temps avant que la grille ne retombe
      (Variables|OPTIONDALLES|Settemps%20avant%20rebaisse 5.0)
      ;;[1 1 1] Gère le temps pendant le quelle la grille n'est pas utilisable
      (Variables|OPTIONDALLES|Settemps%20end-lag 0.0))
    (:NewEnumerator1
      (Variables|OPTIONDALLES|Settemps%20monté 2.5)
      (Variables|OPTIONDALLES|Settemps%20descente 2.0)
      (Variables|OPTIONDALLES|Settemps%20avant%20rebaisse 1.0)
      (Variables|OPTIONDALLES|Settemps%20end-lag 1.0))
    (:NewEnumerator2
      (Variables|OPTIONDALLES|Settemps%20monté 5.0)
      (Variables|OPTIONDALLES|Settemps%20descente 1.0)
      (Variables|OPTIONDALLES|Settemps%20avant%20rebaisse 0.5)
      (Variables|OPTIONDALLES|Settemps%20end-lag 3.0))))

(fn ConstructionScript
  ;[1 1 1] Donne une couleur différente selon la valeur de " type grille "
  (bind _returnvalue (Rendering|Material|CreateDynamicMaterialInstance (Variables|Default|Getgrille) 0 "/Game/_MAIN/MAP/MAP_TEST_LEVEL-DESIGN_ALEX/Matérials/M_grille_lente.M_grille_lente" "None" :!class /Script/Engine.PrimitiveComponent))
  (switch Utilities|FlowControl|Switch|Switchonenum_grille_lente (Variables|Default|GetSelection)
    (:NewEnumerator0
      (Rendering|Material|SetVectorParameterValue _returnvalue "couleur_rouge" "(R=0.000000,G=0.354708,B=1.000000,A=1.000000)" :!class /Script/Engine.MaterialInstanceDynamic))
    (:NewEnumerator1
      (Rendering|Material|SetVectorParameterValue _returnvalue "couleur_rouge" "(R=0.986004,G=1.000000,B=0.000000,A=1.000000)" :!class /Script/Engine.MaterialInstanceDynamic))
    (:NewEnumerator2
      (Rendering|Material|SetVectorParameterValue _returnvalue "couleur_rouge" "(R=1.000000,G=0.016558,B=0.000000,A=1.000000)" :!class /Script/Engine.MaterialInstanceDynamic))))