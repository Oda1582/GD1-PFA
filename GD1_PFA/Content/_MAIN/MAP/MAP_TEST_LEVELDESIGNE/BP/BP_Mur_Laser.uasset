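; BP_Mur_Laser is a laser wall actor that displays seven laser effect components.
; Each laser's "Laser END" vector parameter is set to a world location, mostly from a paired Scene component acting as the beam target.
; Laser6 is the exception, using its own location as the end point.
; The same assignments run in the Construction Script and again on BeginPlay, with no damage or detection logic.
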(event EventBeginPlay
  (Effects|Components|ParticleSystem|SetVectorParameter (Variables|Default|GetLaser) "Laser END" (Transformation|GetWorldLocation (Variables|Default|GetScene)))
  (Effects|Components|ParticleSystem|SetVectorParameter (Variables|Default|GetLaser1) "Laser END" (Transformation|GetWorldLocation (Variables|Default|GetScene1)))
  (Effects|Components|ParticleSystem|SetVectorParameter (Variables|Default|GetLaser2) "Laser END" (Transformation|GetWorldLocation (Variables|Default|GetScene2)))
  (Effects|Components|ParticleSystem|SetVectorParameter (Variables|Default|GetLaser3) "Laser END" (Transformation|GetWorldLocation (Variables|Default|GetScene3)))
  (Effects|Components|ParticleSystem|SetVectorParameter (Variables|Default|GetLaser4) "Laser END" (Transformation|GetWorldLocation (Variables|Default|GetScene4)))
  (Effects|Components|ParticleSystem|SetVectorParameter (Variables|Default|GetLaser5) "Laser END" (Transformation|GetWorldLocation (Variables|Default|GetScene5)))
  (Effects|Components|ParticleSystem|SetVectorParameter (Variables|Default|GetLaser6) "Laser END" (Transformation|GetWorldLocation (Variables|Default|GetLaser6))))

(fn ConstructionScript
  (Effects|Components|ParticleSystem|SetVectorParameter (Variables|Default|GetLaser) "Laser END" (Transformation|GetWorldLocation (Variables|Default|GetScene)))
  (Effects|Components|ParticleSystem|SetVectorParameter (Variables|Default|GetLaser1) "Laser END" (Transformation|GetWorldLocation (Variables|Default|GetScene1)))
  (Effects|Components|ParticleSystem|SetVectorParameter (Variables|Default|GetLaser2) "Laser END" (Transformation|GetWorldLocation (Variables|Default|GetScene2)))
  (Effects|Components|ParticleSystem|SetVectorParameter (Variables|Default|GetLaser3) "Laser END" (Transformation|GetWorldLocation (Variables|Default|GetScene3)))
  (Effects|Components|ParticleSystem|SetVectorParameter (Variables|Default|GetLaser4) "Laser END" (Transformation|GetWorldLocation (Variables|Default|GetScene4)))
  (Effects|Components|ParticleSystem|SetVectorParameter (Variables|Default|GetLaser5) "Laser END" (Transformation|GetWorldLocation (Variables|Default|GetScene5)))
  (Effects|Components|ParticleSystem|SetVectorParameter (Variables|Default|GetLaser6) "Laser END" (Transformation|GetWorldLocation (Variables|Default|GetLaser6))))