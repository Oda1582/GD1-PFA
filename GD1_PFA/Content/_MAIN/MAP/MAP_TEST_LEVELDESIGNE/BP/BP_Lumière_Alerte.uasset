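; A level-design alert light Blueprint that spins a spotlight like an alarm beacon and can switch it on with a sound.
; Every tick, the spotlight yaws in local space at an editable rotation speed scaled by delta time.
; The Allumagelumierealarme event makes the spotlight visible and plays the alert sound cue at its location.
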(event Custom|Allumage%20lumiere%20alarme
  (Rendering|SetVisibility (Variables|Default|GetSpotLight) true false)
  (Audio|PlaySoundatLocation "/Game/_MAIN/Sound/alert-sound_Cue.alert-sound_Cue" (Transformation|GetWorldLocation (Variables|Default|GetSpotLight)) "0, 0, 0" 1.0 1.0 0.0 0 0 0 0))

(event EventTick
  (params (DeltaSeconds :type Float%20%28single-precision%29))
  ;[0 0 0] On créé une rotation sur la spotlight
  (Transformation|AddLocalRotation (Variables|Default|GetSpotLight) (* (Math|Rotator|MakeRotator 0.0 0.0 (Variables|PARAMETTRE|GetVitesse%20de%20rotation)) DeltaSeconds) false false))

(fn ConstructionScript)