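; Physics object for the Physics Gun that highlights when the player aims at it within interaction range.
; Construction script and BeginPlay apply its configurable mesh, material, mass and physics simulation to the Cube.
; Once the rifle is picked up, Tick checks player distance, then sphere-traces from the camera while nothing is grabbed.
; A hit on itself with Physics Gun selected enables the post process and custom depth highlight.
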(event EventBeginPlay
  (Utilities|FlowControl|Sequence
    (:then_0
      (bind _asbp_first_person_character (Utilities|Casting|CastToBP_FirstPersonCharacter (Game|GetPlayerCharacter 0)))
      (Variables|Default|SetPlayer _asbp_first_person_character))
    (:then_1
      (Class|PrimitiveComponent|SetMassOverrideinKg (Variables|Default|GetCube) "None" (Variables|Default|GetMass%20in%20KG) true)
      (Class|PrimitiveComponent|SetMassScale (Variables|Default|GetCube) "None" 1.0)
      (Rendering|Material|SetMaterial (Variables|Default|GetCube) 0 (Variables|Default|GetMaterial))
      (Components|StaticMesh|SetStaticMesh (Variables|Default|GetCube) (Variables|Default|GetMesh))
      (Physics|SetSimulatePhysics (Variables|Default|GetCube) (Variables|Default|GetSimulate%20physics)))))

(event EventTick
  (params (DeltaSeconds :type Float%20%28single-precision%29))
  (bind _player (Variables|Default|GetPlayer))
  (bind _firstpersoncamera (Variables|/Game/FirstPerson/Blueprints/BP_FirstPersonCharacter.BP_FirstPersonCharacter_C|GetFirstPersonCamera _player))
  (bind _returnvalue (Transformation|GetWorldLocation _firstpersoncamera))
  (if (Variables|/Game/FirstPerson/Blueprints/BP_Rifle.BP_Rifle_C|GetPickedUp (Variables|/Game/FirstPerson/Blueprints/BP_FirstPersonCharacter.BP_FirstPersonCharacter_C|GetRifle (Variables|Default|GetPlayer)))
    (Utilities|FlowControl|Sequence
      (:then_0
        (Math|Float|CompareFloat (Transformation|GetDistanceTo (Game|GetPlayerCharacter 0)) (Variables|/Game/FirstPerson/Blueprints/BP_FirstPersonCharacter.BP_FirstPersonCharacter_C|GetInteraction%20Distance (Variables|Default|GetPlayer))
          (:>
            (Variables|Default|SetHighlight false))
          (:<
            (Variables|Default|SetHighlight true))))
      (:then_1
        (if (Variables|Default|GetHighlight)
          (if (Variables|/Game/FirstPerson/Blueprints/BP_FirstPersonCharacter.BP_FirstPersonCharacter_C|GetGrabbed (Variables|Default|GetPlayer))
            (Variables|/Script/Engine.PostProcessComponent|SetbEnabled (Variables|Default|GetPostProcess) false :!label _label)
            (Rendering|SetRenderCustomDepth (Variables|Default|GetCube) false)
            (else
              (bind _outhit (Collision|SphereTraceForObjects _returnvalue (+ _returnvalue (* (Math|Vector|GetForwardVector _firstpersoncamera) (Variables|/Game/FirstPerson/Blueprints/BP_FirstPersonCharacter.BP_FirstPersonCharacter_C|GetInteraction%20Distance (Variables|Default|GetPlayer)))) 2e+01 (Utilities|Array|MakeArray "ObjectTypeQuery4") false (Utilities|Array|MakeArray (Variables|Default|GetPlayer)) "None" false))
              (if (.bBlockingHit (Collision|BreakHitResult _outhit))
                (if (== (.HitActor (Collision|BreakHitResult _outhit)) self)
                  (switch Utilities|FlowControl|Switch|SwitchonBP_ToolGun_Mode (Variables|/Game/FirstPerson/Blueprints/BP_FirstPersonCharacter.BP_FirstPersonCharacter_C|GetSelection (Variables|Default|GetPlayer))
                    (:NewEnumerator0
                      (Variables|/Script/Engine.PostProcessComponent|SetbEnabled (Variables|Default|GetPostProcess) true)
                      (Rendering|SetRenderCustomDepth (Variables|Default|GetCube) true))
                    (:NewEnumerator1
                      (Variables|/Script/Engine.PostProcessComponent|SetbEnabled (Variables|Default|GetPostProcess) false :!label _label_2)
                      (Rendering|SetRenderCustomDepth (Variables|Default|GetCube) false)))
                  (else
                    (goto _label_2)))
                (else
                  (goto _label_2)))))
          (else
            (goto _label)))))))

(event Collision|EventActorBeginOverlap
  (params (OtherActor :type Actor%20Object%20Reference)))

(fn ConstructionScript
  (Class|PrimitiveComponent|SetMassOverrideinKg (Variables|Default|GetCube) "None" (Variables|Default|GetMass%20in%20KG) true)
  (Rendering|Material|SetMaterial (Variables|Default|GetCube) 0 (Variables|Default|GetMaterial))
  (Components|StaticMesh|SetStaticMesh (Variables|Default|GetCube) (Variables|Default|GetMesh))
  (Physics|SetSimulatePhysics (Variables|Default|GetCube) (Variables|Default|GetSimulate%20physics)))