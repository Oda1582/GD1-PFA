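; BP_DoublePorte is an automatic sliding double door that responds to overlaps on a detection sphere.
; Begin overlap slides the two leaf meshes apart with MoveComponentTo over VitesseDouverture, and end overlap slides them back.
; The same overlaps switch a vector in the MCP_DetecteurPorte parameter collection to red on entry and green on exit.
; LockPorte disables the sphere's collision, stopping detection.
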(event OnComponentBeginOverlap(Sphere)
  (params (OverlappedComponent :type Primitive%20Component%20Object%20Reference) (OtherActor :type Actor%20Object%20Reference) (OtherComp :type Primitive%20Component%20Object%20Reference) (OtherBodyIndex :type Integer) (bFromSweep :type Boolean) (SweepResult :type Hit%20Result%20Structure%20%28by%20ref%29))
  (Rendering|Material|SetVectorParameterValue "/Game/_MAIN/Proto_Materials/MCP_DetecteurPorte.MCP_DetecteurPorte" "Vector" (Utilities|Struct|MakeLinearColor 1.0 0.0 0.0 0.0) :!class /Script/Engine.KismetMaterialLibrary)
  (CallFunction|PorteDroite)
  (CallFunction|PorteGauche))

(event OnComponentEndOverlap(Sphere)
  (params (OverlappedComponent :type Primitive%20Component%20Object%20Reference) (OtherActor :type Actor%20Object%20Reference) (OtherComp :type Primitive%20Component%20Object%20Reference) (OtherBodyIndex :type Integer))
  (Rendering|Material|SetVectorParameterValue "/Game/_MAIN/Proto_Materials/MCP_DetecteurPorte.MCP_DetecteurPorte" "Vector" (Utilities|Struct|MakeLinearColor 0.0 1.0 0.0 0.0) :!class /Script/Engine.KismetMaterialLibrary)
  (CallFunction|FermeturePorteDroite)
  (CallFunction|FermeturePorteGauche))

(event Custom|Porte%20Droite
  (Components|MoveComponentTo (Variables|Default|GetSM_Porte) "0,150.000000,110.000000" "0, 0, 0" false false (Variables|Default|GetVitesse%20d'ouverture) false))

(event Custom|Porte%20gauche
  (Components|MoveComponentTo (Variables|Default|GetSM_Porte1) "0,-150.000000,110.000000" "0, 0, 0" false false (Variables|Default|GetVitesse%20d'ouverture) false))

(event Custom|Fermeture%20Porte%20Droite
  (Components|MoveComponentTo (Variables|Default|GetSM_Porte) "0,50.000000,110.000000" "0, 0, 0" false false (Variables|Default|GetVitesse%20d'ouverture) false))

(event Custom|Fermeture%20Porte%20Gauche
  (Components|MoveComponentTo (Variables|Default|GetSM_Porte1) "0,-50.000000,110.000000" "0, 0, 0" false false (Variables|Default|GetVitesse%20d'ouverture) false))

(event Custom|LockPorte
  (Collision|SetCollisionEnabled (Variables|Default|GetSphere) "NoCollision"))

(fn ConstructionScript)