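; Automatic sliding metal door that opens when the first-person character enters its Box trigger and closes when they leave.
; MoveComponentTo slides PorteMetal to the Scene component's relative location to open and to a hardcoded position to close.
; Two cross-resetting DoOnce nodes alternate the moves, each re-arming the other after its move completes.
; Every character entry or exit spawns the same door sound at the actor's location, independent of those gates.
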(event OnComponentBeginOverlap(Box)
  (params (OverlappedComponent :type Primitive%20Component%20Object%20Reference) (OtherActor :type Actor%20Object%20Reference) (OtherComp :type Primitive%20Component%20Object%20Reference) (OtherBodyIndex :type Integer) (bFromSweep :type Boolean) (SweepResult :type Hit%20Result%20Structure%20%28by%20ref%29))
  (Utilities|Casting|CastToBP_FirstPersonCharacter OtherActor)
  (Utilities|FlowControl|Sequence
    (:then_0
      (Utilities|FlowControl|DoOnce false
        (:Completed
          (Components|MoveComponentTo (Variables|Default|GetPorte_metal) (Variables|/Script/Engine.SceneComponent|GetRelativeLocation (Variables|Default|GetScene)) (Variables|/Script/Engine.SceneComponent|GetRelativeRotation (Variables|Default|GetPorte_metal)) false false 0.6 true)
          (Utilities|FlowControl|DoOnce false) ; enters at Reset
        )))
    (:then_1
      (Audio|SpawnSoundatLocation "/Game/_MAIN/Sound/automatic-electric-door-open-sound-effects-short-to-long-tone_rUjvODLG_Cue.automatic-electric-door-open-sound-effects-short-to-long-tone_rUjvODLG_Cue" (Transformation|GetActorLocation) "0, 0, 0" 1.0 1.0 0.2 0 0))))

(event OnComponentEndOverlap(Box)
  (params (OverlappedComponent :type Primitive%20Component%20Object%20Reference) (OtherActor :type Actor%20Object%20Reference) (OtherComp :type Primitive%20Component%20Object%20Reference) (OtherBodyIndex :type Integer))
  (Utilities|Casting|CastToBP_FirstPersonCharacter OtherActor)
  (Utilities|FlowControl|Sequence
    (:then_0
      (Utilities|FlowControl|DoOnce false
        (:Completed
          (Components|MoveComponentTo (Variables|Default|GetPorte_metal) "13.071442,-0.000002,0.000000" (Variables|/Script/Engine.SceneComponent|GetRelativeRotation (Variables|Default|GetPorte_metal)) false false 0.6 true)
          (Utilities|FlowControl|DoOnce false) ; enters at Reset
        )))
    (:then_1
      (Audio|SpawnSoundatLocation "/Game/_MAIN/Sound/automatic-electric-door-open-sound-effects-short-to-long-tone_rUjvODLG_Cue.automatic-electric-door-open-sound-effects-short-to-long-tone_rUjvODLG_Cue" (Transformation|GetActorLocation) "0, 0, 0" 1.0 1.0 0.2 0 0))))

(event EventBeginPlay)

(event Collision|EventActorBeginOverlap
  (params (OtherActor :type Actor%20Object%20Reference)))

(event EventTick
  (params (DeltaSeconds :type Float%20%28single-precision%29)))

(fn ConstructionScript)