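; Flickering neon light Blueprint that toggles its point light on and off at random intervals from BeginPlay.
; A random delay of a few seconds feeds a FlipFlop, then the update_flick event restarts the cycle.
; Switching off plays a sound at the light's location.
; Each state also sets a neon scalar in the MCP_DetecteurPorte Material Parameter Collection, so materials reading it follow the flicker.
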(event Custom|update_flick
  (bind _pointlight (Variables|Default|GetPointLight))
  ;[1 1 1] relance le système à la fin de chaque cycle
  ;[1 1 1] Gestion du temps aléatoire
  (Utilities|FlowControl|Delay (Math|Random|RandomFloatinRange 1.0 3.0))
  (Utilities|FlowControl|FlipFlop
    (:A
      ;[1 1 1] Fait le bruitage  à chaque fois qu'elle s'éteint
      (Audio|PlaySoundatLocation "/Game/_MAIN/HUD/Sons/ARGH.ARGH" (Transformation|GetWorldLocation _pointlight) "0, 0, 0" 1.0 1.0 0.0 0 0 0 0)
      ;[1 1 1] Plus visible / Visible
      (Rendering|SetVisibility _pointlight false false)
      (Rendering|Material|SetScalarParameterValue "/Game/_MAIN/Proto_Materials/MCP_DetecteurPorte.MCP_DetecteurPorte" "Scalar_BP_néon" 0.0 :!class /Script/Engine.KismetMaterialLibrary))
    (:B
      (Rendering|SetVisibility _pointlight true false)
      (Rendering|Material|SetScalarParameterValue "/Game/_MAIN/Proto_Materials/MCP_DetecteurPorte.MCP_DetecteurPorte" "Scalar_BP_néon" 5e+01 :!class /Script/Engine.KismetMaterialLibrary)))
  (CallFunction|UpdateFlick))

(event EventBeginPlay
  (bind _pointlight (Variables|Default|GetPointLight))
  ;[1 1 1] Gestion du temps aléatoire
  (Utilities|FlowControl|Delay (Math|Random|RandomFloatinRange 1.0 3.0))
  (Utilities|FlowControl|FlipFlop
    (:A
      ;[1 1 1] Fait le bruitage  à chaque fois qu'elle s'éteint
      (Audio|PlaySoundatLocation "/Game/_MAIN/HUD/Sons/ARGH.ARGH" (Transformation|GetWorldLocation _pointlight) "0, 0, 0" 1.0 1.0 0.0 0 0 0 0)
      ;[1 1 1] Plus visible / Visible
      (Rendering|SetVisibility _pointlight false false)
      (Rendering|Material|SetScalarParameterValue "/Game/_MAIN/Proto_Materials/MCP_DetecteurPorte.MCP_DetecteurPorte" "Scalar_BP_néon" 0.0 :!class /Script/Engine.KismetMaterialLibrary))
    (:B
      (Rendering|SetVisibility _pointlight true false)
      (Rendering|Material|SetScalarParameterValue "/Game/_MAIN/Proto_Materials/MCP_DetecteurPorte.MCP_DetecteurPorte" "Scalar_BP_néon" 5e+01 :!class /Script/Engine.KismetMaterialLibrary)))
  (CallFunction|UpdateFlick))

(fn ConstructionScript)