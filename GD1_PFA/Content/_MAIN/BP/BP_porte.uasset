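; BP_porte is an automatic double door that opens when the first-person character enters its Box trigger and closes when they leave.
; Opening moves both panels over a fixed duration to the SceneGauche and SceneDroite component positions, while closing returns them to hardcoded relative locations.
; Both events use MoveComponentTo, keep each panel's rotation, and spawn their own sound at the actor's location.
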(event OnComponentBeginOverlap(Box)
  (params (OverlappedComponent :type Primitive%20Component%20Object%20Reference) (OtherActor :type Actor%20Object%20Reference) (OtherComp :type Primitive%20Component%20Object%20Reference) (OtherBodyIndex :type Integer) (bFromSweep :type Boolean) (SweepResult :type Hit%20Result%20Structure%20%28by%20ref%29))
  (Utilities|Casting|CastToBP_FirstPersonCharacter OtherActor)
  (CallFunction|OuvrirPorte))

(event OnComponentEndOverlap(Box)
  (params (OverlappedComponent :type Primitive%20Component%20Object%20Reference) (OtherActor :type Actor%20Object%20Reference) (OtherComp :type Primitive%20Component%20Object%20Reference) (OtherBodyIndex :type Integer))
  (Utilities|Casting|CastToBP_FirstPersonCharacter OtherActor)
  (CallFunction|FermerPorte))

(event Custom|Ouvrir%20porte
  (bind _porte_gauche (Variables|Default|GetPorte%20Gauche))
  (bind _porte_droite (Variables|Default|GetPorte%20Droite))
  (Utilities|FlowControl|Sequence
    (:then_0
      (Components|MoveComponentTo _porte_gauche (Variables|/Script/Engine.SceneComponent|GetRelativeLocation (Variables|Default|GetScene%20gauche)) (Variables|/Script/Engine.SceneComponent|GetRelativeRotation _porte_gauche) false false 1.5 false))
    (:then_1
      (Components|MoveComponentTo _porte_droite (Variables|/Script/Engine.SceneComponent|GetRelativeLocation (Variables|Default|GetScene%20droite)) (Variables|/Script/Engine.SceneComponent|GetRelativeRotation _porte_droite) false false 1.5 false))
    (:then_2
      (Audio|SpawnSoundatLocation "/Game/_MAIN/Sound/automatic-electric-door-open-sound-effects-short-to-long-tone_rUjvODLG_Cue.automatic-electric-door-open-sound-effects-short-to-long-tone_rUjvODLG_Cue" (Transformation|GetActorLocation) "0, 0, 0" 1.0 1.0 0.2 0 0))))

(event Custom|Fermer%20porte
  (bind _porte_gauche (Variables|Default|GetPorte%20Gauche))
  (bind _porte_droite (Variables|Default|GetPorte%20Droite))
  (Utilities|FlowControl|Sequence
    (:then_0
      (Components|MoveComponentTo _porte_gauche "-116.394745,-7.031879, 0" (Variables|/Script/Engine.SceneComponent|GetRelativeRotation _porte_gauche) false false 1.5 false))
    (:then_1
      (Components|MoveComponentTo _porte_droite "110.734650,0.000000, 0" (Variables|/Script/Engine.SceneComponent|GetRelativeRotation _porte_droite) false false 1.5 false))
    (:then_2
      (Audio|SpawnSoundatLocation "/Game/_MAIN/Sound/Porte_Ascenceur_Cue.Porte_Ascenceur_Cue" (Transformation|GetActorLocation) "0, 0, 0" 1.0 1.0 0.2 0 0))))

(event EventBeginPlay)

(event Collision|EventActorBeginOverlap
  (params (OtherActor :type Actor%20Object%20Reference)))

(event EventTick
  (params (DeltaSeconds :type Float%20%28single-precision%29)))

(fn ConstructionScript)