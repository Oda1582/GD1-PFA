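; BP_Rect_Light is a configurable rect light fixture that pairs a RectLight component with a Cube mesh component.
; The construction script applies variables for attenuation radius, color, barn door angle, intensity and shadow casting to the light, and sets the cube's mesh and first material.
; BeginPlay reapplies the same light settings except shadow casting, and leaves the mesh and material untouched.
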(event EventBeginPlay
  (Rendering|Lighting|SetAttenuationRadius (Variables|Default|GetRectLight) (Variables|Default|GetAttenuation%20Radius))
  (Rendering|Components|Light|SetLightColor (Variables|Default|GetRectLight) (Variables|Default|GetLight%20Color) true)
  (Class|RectLightComponent|SetBarnDoorAngle (Variables|Default|GetRectLight) (Variables|Default|GetBarn%20Door%20Angle))
  (Rendering|Components|Light|SetIntensity (Variables|Default|GetRectLight) (Variables|Default|GetIntensity)))

(event Collision|EventActorBeginOverlap
  (params (OtherActor :type Actor%20Object%20Reference)))

(event EventTick
  (params (DeltaSeconds :type Float%20%28single-precision%29)))

(fn ConstructionScript
  (bind _cube (Variables|Default|GetCube))
  (Rendering|Lighting|SetAttenuationRadius (Variables|Default|GetRectLight) (Variables|Default|GetAttenuation%20Radius))
  (Rendering|Components|Light|SetLightColor (Variables|Default|GetRectLight) (Variables|Default|GetLight%20Color) true)
  (Class|RectLightComponent|SetBarnDoorAngle (Variables|Default|GetRectLight) (Variables|Default|GetBarn%20Door%20Angle))
  (Rendering|Components|Light|SetIntensity (Variables|Default|GetRectLight) (Variables|Default|GetIntensity))
  (Rendering|Components|Light|SetCastShadows (Variables|Default|GetRectLight) (Variables|Default|GetCast%20Shadow))
  (Components|StaticMesh|SetStaticMesh _cube (Variables|Default|GetMesh))
  (Rendering|Material|SetMaterial _cube 0 (Variables|Default|GetMaterial)))