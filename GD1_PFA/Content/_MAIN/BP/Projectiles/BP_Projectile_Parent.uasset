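; Base projectile actor that damages the first-person player character when it hits them.
; On BeginPlay it copies its gravity, initial speed and max speed variables into the ProjectileMovement component.
; When its Sphere hits anything, it applies DamageProjectile only to BP_FirstPersonCharacter, then always spawns a Niagara hit effect, plays a 2D sound and destroys itself.
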(event OnComponentHit(Sphere)
  (params (HitComponent :type Primitive%20Component%20Object%20Reference) (OtherActor :type Actor%20Object%20Reference) (OtherComp :type Primitive%20Component%20Object%20Reference) (NormalImpulse :type Vector :default "0, 0, 0") (Hit :type Hit%20Result%20Structure%20%28by%20ref%29))
  (Utilities|FlowControl|Sequence
    (:then_0
      (bind _asbp_first_person_character (Utilities|Casting|CastToBP_FirstPersonCharacter OtherActor))
      (Game|Damage|ApplyDamage _asbp_first_person_character (Variables|Default|GetDamageProjectile) 0 0))
    (:then_1
      (Niagara|SpawnSystematLocation (Variables|Default|GetNS%20Hit) (Transformation|GetActorLocation))
      (Audio|SpawnSound2D (Variables|Default|GetSound%20Hit) 1.0 1.0 0.0 0)
      ;[1 1 1] Gêne ralentissement ?
      (Actor|DestroyActor))))

(event EventBeginPlay
  (bind _projectilemovement (Variables|Default|GetProjectileMovement))
  (Variables|/Script/Engine.ProjectileMovementComponent|SetProjectileGravityScale _projectilemovement (Variables|Default|GetProjectileGravity))
  (Variables|/Script/Engine.ProjectileMovementComponent|SetInitialSpeed _projectilemovement (Variables|Default|GetProjectileInitialSpeed))
  (Variables|/Script/Engine.ProjectileMovementComponent|SetMaxSpeed _projectilemovement (Variables|Default|GetProjectileMaxSpeed)))

(fn ConstructionScript)