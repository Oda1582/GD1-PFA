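; Flickering rect light actor whose radius, color, barn door angle, intensity and shadow casting are set from variables.
; On BeginPlay it starts an endless loop: a random delay, then a FlipFlop toggles visibility, and a custom event re-enters the delay.
; Switching off plays a quiet sound at the light.
; Each toggle also writes a neon scalar in the MCP_DetecteurPorte parameter collection, keeping it in step with the light.
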(event Custom|update_flick_rec
  (bind _rectlight (Variables|Default|GetRectLight))
  ;[1 1 1] relance le système à la fin de chaque cycle
  ;[1 1 1] Gestion du temps aléatoire
  (Utilities|FlowControl|Delay (Math|Random|RandomFloatinRange 0.5 2.0))
  (Utilities|FlowControl|FlipFlop
    (:A
      ;[1 1 1] Fait le bruitage  à chaque fois qu'elle s'éteint
      (Audio|PlaySoundatLocation 0 (Transformation|GetWorldLocation _rectlight) "0, 0, 0" 0.2 1.0 0.0 0 0 0 0)
      ;[1 1 1] Plus visible / Visible
      (Rendering|SetVisibility _rectlight false false)
      (Rendering|Material|SetScalarParameterValue "/Game/_MAIN/Proto_Materials/MCP_DetecteurPorte.MCP_DetecteurPorte" "Scalar_BP_néon" 0.0 :!class /Script/Engine.KismetMaterialLibrary))
    (:B
      (Rendering|SetVisibility _rectlight true false)
      (Rendering|Material|SetScalarParameterValue "/Game/_MAIN/Proto_Materials/MCP_DetecteurPorte.MCP_DetecteurPorte" "Scalar_BP_néon" 5e+01 :!class /Script/Engine.KismetMaterialLibrary)))
  (CallFunction|UpdateFlickRec))

(event EventBeginPlay
  (bind _rectlight (Variables|Default|GetRectLight))
  (Utilities|FlowControl|Sequence
    (:then_0
      (Rendering|Lighting|SetAttenuationRadius (Variables|Default|GetRectLight) (Variables|Default|GetAttenuation%20Radius))
      (Rendering|Components|Light|SetLightColor (Variables|Default|GetRectLight) (Variables|Default|GetLight%20Color) true)
      (Class|RectLightComponent|SetBarnDoorAngle (Variables|Default|GetRectLight) (Variables|Default|GetBarn%20Door%20Angle))
      (Rendering|Components|Light|SetIntensity (Variables|Default|GetRectLight) (Variables|Default|GetIntensity)))
    (:then_1
      ;[1 1 1] Gestion du temps aléatoire
      (Utilities|FlowControl|Delay (Math|Random|RandomFloatinRange 0.5 2.0))
      (Utilities|FlowControl|FlipFlop
        (:A
          ;[1 1 1] Fait le bruitage  à chaque fois qu'elle s'éteint
          (Audio|PlaySoundatLocation 0 (Transformation|GetWorldLocation _rectlight) "0, 0, 0" 0.2 1.0 0.0 0 0 0 0)
          ;[1 1 1] Plus visible / Visible
          (Rendering|SetVisibility _rectlight false false)
          (Rendering|Material|SetScalarParameterValue "/Game/_MAIN/Proto_Materials/MCP_DetecteurPorte.MCP_DetecteurPorte" "Scalar_BP_néon" 0.0 :!class /Script/Engine.KismetMaterialLibrary))
        (:B
          (Rendering|SetVisibility _rectlight true false)
          (Rendering|Material|SetScalarParameterValue "/Game/_MAIN/Proto_Materials/MCP_DetecteurPorte.MCP_DetecteurPorte" "Scalar_BP_néon" 5e+01 :!class /Script/Engine.KismetMaterialLibrary)))
      (CallFunction|UpdateFlickRec))))

(fn ConstructionScript
  (Rendering|Lighting|SetAttenuationRadius (Variables|Default|GetRectLight) (Variables|Default|GetAttenuation%20Radius))
  (Rendering|Components|Light|SetLightColor (Variables|Default|GetRectLight) (Variables|Default|GetLight%20Color) true)
  (Class|RectLightComponent|SetBarnDoorAngle (Variables|Default|GetRectLight) (Variables|Default|GetBarn%20Door%20Angle))
  (Rendering|Components|Light|SetIntensity (Variables|Default|GetRectLight) (Variables|Default|GetIntensity))
  (Rendering|Components|Light|SetCastShadows (Variables|Default|GetRectLight) (Variables|Default|GetCast%20Shadow)))