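; Elevator actor with two sliding doors that acts as a transition to another level.
; Ouvrirporte slides both doors to scene-component markers with MoveComponentTo, playing a door sound that is later stopped and a delayed arrival ring.
; Fermerporte slides them to hardcoded closed positions with the door sound, then opens the referenced Level shortly after the left door finishes moving.
; Nothing in this Blueprint triggers either event; an open-wait-close chain is left disconnected.
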(event Custom|Ouvrir%20porte
  (bind _porte_gauche (Variables|Default|GetPorte%20Gauche))
  (bind _porte_droite (Variables|Default|GetPorte%20Droite))
  (Utilities|FlowControl|Sequence
    (:then_0
      (Components|MoveComponentTo _porte_gauche (Variables|/Script/Engine.SceneComponent|GetRelativeLocation (Variables|Default|GetScene%20gauche)) (Variables|/Script/Engine.SceneComponent|GetRelativeRotation _porte_gauche) false false 1.5 false))
    (:then_1
      (Components|MoveComponentTo _porte_droite (Variables|/Script/Engine.SceneComponent|GetRelativeLocation (Variables|Default|GetScene%20droite)) (Variables|/Script/Engine.SceneComponent|GetRelativeRotation _porte_droite) false false 1.5 false))
    (:then_2
      (bind _returnvalue (Audio|SpawnSoundatLocation "/Game/_MAIN/Sound/Porte_Ascenceur_Cue.Porte_Ascenceur_Cue" (Transformation|GetActorLocation) "0, 0, 0" 1.0 1.0 0.2 0 0))
      (Utilities|FlowControl|Sequence
        (:then_0
          (Utilities|FlowControl|Delay 1.5)
          (Audio|Components|Audio|Stop _returnvalue))
        (:then_1
          (Utilities|FlowControl|Delay 0.7)
          (Audio|SpawnSoundatLocation "/Game/_MAIN/Sound/Ring_Ascenceur_Cue.Ring_Ascenceur_Cue" (Transformation|GetActorLocation) "0, 0, 0" 1.0 1.0 0.0 0 0))))))

(event Custom|Fermer%20porte
  (bind _porte_gauche (Variables|Default|GetPorte%20Gauche))
  (bind _porte_droite (Variables|Default|GetPorte%20Droite))
  (Utilities|FlowControl|Sequence
    (:then_0
      (Components|MoveComponentTo _porte_gauche "50.661873,-358.000000, 0" (Variables|/Script/Engine.SceneComponent|GetRelativeRotation _porte_gauche) false false 1.5 false)
      (Utilities|FlowControl|Delay 0.6)
      (Game|OpenLevel(byObjectReference) (Variables|Default|GetLevel)))
    (:then_1
      (Components|MoveComponentTo _porte_droite "-111.470718,-341.000000, 0" (Variables|/Script/Engine.SceneComponent|GetRelativeRotation _porte_droite) false false 1.5 false))
    (:then_2
      (Audio|SpawnSoundatLocation "/Game/_MAIN/Sound/Porte_Ascenceur_Cue.Porte_Ascenceur_Cue" (Transformation|GetActorLocation) "0, 0, 0" 1.0 1.0 0.2 0 0))))

(event EventBeginPlay)

(event Collision|EventActorBeginOverlap
  (params (OtherActor :type Actor%20Object%20Reference)))

(event EventTick
  (params (DeltaSeconds :type Float%20%28single-precision%29)))

(fn ConstructionScript)