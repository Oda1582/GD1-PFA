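; BP_Podium is a podium that takes two kinds of magnetic card objects, standard and blue, when they overlap its box.
; Each card lights its own mesh's emissive parameter, increments an Objectif counter, deactivates the player's PG, stops its sound and is destroyed.
; The standard card also sets every BP_Rect_Light in the level to zero intensity.
; Both card meshes start unlit on BeginPlay; nothing here reads Objectif.
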(event OnComponentBeginOverlap(Box)
  (params (OverlappedComponent :type Primitive%20Component%20Object%20Reference) (OtherActor :type Actor%20Object%20Reference) (OtherComp :type Primitive%20Component%20Object%20Reference) (OtherBodyIndex :type Integer) (bFromSweep :type Boolean) (SweepResult :type Hit%20Result%20Structure%20%28by%20ref%29))
  (bind _asbp_objet_pg_v_2_carte_magnetique (Utilities|Casting|CastToBP_Objet_PG_v2_carte_magnetique OtherActor)
    (:then
      (Rendering|Material|SetScalarParameterValueonMaterials (Variables|Default|GetSM_CarteAcces) "Emissive" 1e+01)
      (bind _result (Math|Float|IncrementFloat (Variables|Default|GetObjectif))
        (:%20%20
          (Variables|Default|SetObjectif _result)
          (bind _asbp_first_person_character (Utilities|Casting|CastToBP_FirstPersonCharacter (Game|GetPlayerCharacter 0)))
          (Default|DeactivatePG _asbp_first_person_character)
          (Utilities|FlowControl|Sequence
            (:then_0
              (Utilities|IsValid (Variables|/Game/FirstPerson/Blueprints/BP_FirstPersonCharacter.BP_FirstPersonCharacter_C|GetSon%20PG _asbp_first_person_character)
                (:Is%20Valid
                  (Audio|Components|Audio|Stop (Variables|/Game/FirstPerson/Blueprints/BP_FirstPersonCharacter.BP_FirstPersonCharacter_C|GetSon%20PG _asbp_first_person_character)))))
            (:then_1
              (Actor|DestroyActor _asbp_objet_pg_v_2_carte_magnetique))
            (:then_2
              (bind _asbp_first_person_character_2 (Utilities|Casting|CastToBP_FirstPersonCharacter (Game|GetPlayerCharacter 0)))
              (Default|DeactivatePG _asbp_first_person_character_2)
              (bind _outactors (Actor|GetAllActorsOfClass "/Game/_MAIN/BP/BP_Rect_Light.BP_Rect_Light_C"))
              (bind _output_get (Variables|Default|SetRect%20light%20array _outactors))
              (for _array_element _output_get
                (bind _output_get_2 (Variables|Default|SetRect%20light _array_element))
                (Rendering|Components|Light|SetIntensity (Variables|/Game/_MAIN/BP/BP_Rect_Light.BP_Rect_Light_C|GetRectLight _output_get_2) 0.0)
                (Utilities|IsValid (Variables|/Game/FirstPerson/Blueprints/BP_FirstPersonCharacter.BP_FirstPersonCharacter_C|GetSon%20PG _asbp_first_person_character_2)
                  (:Is%20Valid
                    (Audio|Components|Audio|Stop (Variables|/Game/FirstPerson/Blueprints/BP_FirstPersonCharacter.BP_FirstPersonCharacter_C|GetSon%20PG _asbp_first_person_character_2))))))))))
    (:CastFailed
      (bind _asbp_objet_pg_v_2_carte_magnetiquebleu (Utilities|Casting|CastToBP_Objet_PG_v2_carte_magnetiquebleu OtherActor))
      (Rendering|Material|SetScalarParameterValueonMaterials (Variables|Default|GetSM_CarteAcces1) "Emissive" 1e+01)
      (bind _result_2 (Math|Float|IncrementFloat (Variables|Default|GetObjectif))
        (:%20%20
          (Variables|Default|SetObjectif _result_2)
          (bind _asbp_first_person_character_3 (Utilities|Casting|CastToBP_FirstPersonCharacter (Game|GetPlayerCharacter 0)))
          (Default|DeactivatePG _asbp_first_person_character_3)
          (Utilities|FlowControl|Sequence
            (:then_0
              (Utilities|IsValid (Variables|/Game/FirstPerson/Blueprints/BP_FirstPersonCharacter.BP_FirstPersonCharacter_C|GetSon%20PG _asbp_first_person_character_3)
                (:Is%20Valid
                  (Audio|Components|Audio|Stop (Variables|/Game/FirstPerson/Blueprints/BP_FirstPersonCharacter.BP_FirstPersonCharacter_C|GetSon%20PG _asbp_first_person_character_3)))))
            (:then_1
              (Actor|DestroyActor _asbp_objet_pg_v_2_carte_magnetiquebleu))))))))

(event EventBeginPlay
  (Rendering|Material|SetScalarParameterValueonMaterials (Variables|Default|GetSM_CarteAcces) "Emissive" 0.0)
  (Rendering|Material|SetScalarParameterValueonMaterials (Variables|Default|GetSM_CarteAcces1) "Emissive" 0.0))

(fn ConstructionScript)