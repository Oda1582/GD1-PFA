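; BP_Girophare is a beacon light actor (girophare) built around a SpotLight component.
; Its construction script applies the exposed attenuation radius, color, intensity and shadow-casting variables to the spotlight, so each instance is configured at construction.
; The event graph holds only disabled default events, so no gameplay or rotation logic runs there.
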(event EventBeginPlay)

(event Collision|EventActorBeginOverlap
  (params (OtherActor :type Actor%20Object%20Reference)))

(event EventTick
  (params (DeltaSeconds :type Float%20%28single-precision%29)))

(fn ConstructionScript
  (Rendering|Lighting|SetAttenuationRadius (Variables|Default|GetSpotLight) (Variables|Default|GetAttenuation%20Radius))
  (Rendering|Components|Light|SetLightColor (Variables|Default|GetSpotLight) (Variables|Default|GetLight%20Color) true)
  (Rendering|Components|Light|SetIntensity (Variables|Default|GetSpotLight) (Variables|Default|GetIntensity))
  (Rendering|Components|Light|SetCastShadows (Variables|Default|GetSpotLight) (Variables|Default|GetCast%20Shadow)))