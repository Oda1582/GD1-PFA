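; Enemy security camera that sweeps its patrol arc, spots the player and raises an alarm through noise events.
; Cone overlap starts a looping sight-trace timer; confirmed sight drives timeline tracking, with a child laser colored for patrolling, cautious or attacking.
; Stun and shield events suspend detection, and Tick outlines jammer cameras under the player's aim when Brouilleur/Shield is selected.
; Also carries turret-style target selection and projectile firing, plus several disconnected leftovers.
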(event OnComponentBeginOverlap(Trigger)
  (params (OverlappedComponent :type Primitive%20Component%20Object%20Reference) (OtherActor :type Actor%20Object%20Reference) (OtherComp :type Primitive%20Component%20Object%20Reference) (OtherBodyIndex :type Integer) (bFromSweep :type Boolean) (SweepResult :type Hit%20Result%20Structure%20%28by%20ref%29)))

(event OnComponentEndOverlap(Trigger)
  (params (OverlappedComponent :type Primitive%20Component%20Object%20Reference) (OtherActor :type Actor%20Object%20Reference) (OtherComp :type Primitive%20Component%20Object%20Reference) (OtherBodyIndex :type Integer)))

(event OnComponentBeginOverlap(Cone)
  (params (OverlappedComponent :type Primitive%20Component%20Object%20Reference) (OtherActor :type Actor%20Object%20Reference) (OtherComp :type Primitive%20Component%20Object%20Reference) (OtherBodyIndex :type Integer) (bFromSweep :type Boolean) (SweepResult :type Hit%20Result%20Structure%20%28by%20ref%29))
  (if (== OtherActor (Variables|Default|GetPlayer))
    (if (not (Variables|Default|GetStun))
      (Variables|Default|SetOther%20Actor OtherActor)
      (bind (_blocking_hit _outhit) (CallFunction|TestTrace))
      (if _blocking_hit
        (if (== (.HitActor (Collision|BreakHitResult _outhit)) (Variables|Default|GetPlayer))
          (bind _returnvalue (Utilities|Time|SetTimerbyEvent (delegate Custom|LookForTarget) 0.1 true))
          (Variables|Default|SetClear%20Timer _returnvalue))))))

(event OnComponentEndOverlap(Cone)
  (params (OverlappedComponent :type Primitive%20Component%20Object%20Reference) (OtherActor :type Actor%20Object%20Reference) (OtherComp :type Primitive%20Component%20Object%20Reference) (OtherBodyIndex :type Integer))
  (if (== OtherActor (Variables|Default|GetPlayer))
    (if (not (Variables|Default|GetStun))
      (Utilities|Time|ClearandInvalidateTimerbyHandle (Variables|Default|GetClear%20Timer))
      (CallFunction|RestartSweep))))

(event Custom|LookForTarget
  (if (not (Variables|Default|GetStun))
    (bind _outhit (CallFunction|TestTrace))
    (if (.bBlockingHit (Collision|BreakHitResult _outhit))
      (if (== (.HitActor (Collision|BreakHitResult _outhit)) (Variables|Default|GetPlayer))
        (Utilities|FlowControl|Sequence
          (:then_0
            (goto _label_2 Reset))
          (:then_1
            (bind _newtrack_0 (Timeline|ReturnToSweep Stop)
              (:Update
                (Transformation|SetRelativeRotation (Variables|Default|GetCanon%20rot-xy) (Math|Rotator|Lerp(Rotator) (Variables|Default|GetLastSeenRotation) "0, 0, 0" _newtrack_0) false false)
                (CallFunction|ChangeState "NewEnumerator0")
                (bind _newtrack_0_2 (Timeline|CameraSweep PlayFromStart)
                  (:Update
                    (CallFunction|ChangeState "NewEnumerator0")
                    (Transformation|SetRelativeRotation (Variables|Default|GetCanon%20rot-xy) (Math|Rotator|MakeRotator 0.0 (Variables|Default|GetAngle%20Y) (Math|Float|Lerp 0.0 5e+01 _newtrack_0_2)) false false))))))
          (:then_2
            (Timeline|CameraSweep Stop))
          (:then_4
            (Variables|Default|SetTarget_Turret (.HitActor (Collision|BreakHitResult _outhit)))
            (Timeline|FollowTarget PlayFromStart
              (:Update
                (if (not (Variables|Default|GetStun))
                  (Utilities|FlowControl|Sequence
                    (:then_0
                      (CallFunction|Lookat)
                      (Utilities|FlowControl|DoOnce false :!label _label
                        (:Completed
                          (CallFunction|ChangeState "NewEnumerator1")
                          (Utilities|FlowControl|Delay 0.5)
                          (Utilities|IsValid (Variables|Default|GetTarget_Turret)
                            (:Is%20Valid
                              (Variables|Default|SetAttack%20Mode true))))))
                    (:then_1
                      (if (Variables|Default|GetAttack%20Mode)
                        (CallFunction|ChangeState "NewEnumerator2")
                        (Utilities|FlowControl|Delay (Variables|Default|GetVitesse%20de%20tir))
                        (Utilities|IsValid (Variables|Default|GetTarget_Turret)
                          (:Is%20Valid
                            (bind _outhit_2 (Collision|LineTraceByChannel (Transformation|GetSocketLocation (Variables|Default|GetCanon%20rot-xy) "Pan") (Math|Vector|RotateVector (Transformation|GetActorLocation (Variables|Default|GetTarget_Turret)) (Math|Rotator|MakeRotator (Math|Random|RandomFloatinRange -2.0 2.0) 0.0 (Math|Random|RandomFloatinRange -2.0 2.0))) "TraceTypeQuery1" false (Utilities|Array|MakeArray self 0) "None"))
                            (Class|AISenseHearing|ReportNoiseEvent (.TraceEnd (Collision|BreakHitResult _outhit_2)) 1.0 (Variables|Default|GetPlayer) 0.0 "None")))))))))))
        (else
          (CallFunction|ChangeState "NewEnumerator1")
          (Utilities|FlowControl|Sequence
            (:then_0
              (Utilities|FlowControl|DoOnce false :!label _label_2
                (:Completed
                  (Variables|Default|SetLastSeenRotation (Variables|/Script/Engine.SceneComponent|GetRelativeRotation (Variables|Default|GetCanon%20rot-xy)))
                  (Timeline|ReturnToSweep PlayFromStart))))
            (:then_1
              (Timeline|FollowTarget Stop))
            (:then_2
              (Variables|Default|SetTarget_Turret 0))
            (:then_3
              (Variables|Default|SetAttack%20Mode false)
              (goto _label Reset))))))))

(event Custom|End
  (params (NewParam :type Actor%20Object%20Reference))
  (bind _targetinrange (Variables|Default|GetTargetInRange))
  ;[1 1 1] Détection de l'ennemi
  (bind _asbp_first_person_character (Utilities|Casting|CastToBP_FirstPersonCharacter (Game|GetPlayerCharacter 0)))
  (if (Utilities|Array|ContainsItem _targetinrange _asbp_first_person_character)
    (Utilities|Array|RemoveItem _targetinrange _asbp_first_person_character)
    (if (== (Variables|Default|GetTargetEnnemyDetected) _asbp_first_person_character)
      (Variables|Default|SetTargetEnnemyDetected 0)
      (CallFunction|SelectTarget)
      ;[1 1 1] Gestion de l'emissive
      (Rendering|Material|SetScalarParameterValueonMaterials (Variables|Default|GetCanon%20rot-xy) "Emissive" 0.0))))

(event Custom|Stop%20Reset
  (bind _returnvalue (Utilities|Time|GetWorldDeltaSeconds))
  (bind _returnvalue_2 (Utilities|Time|GetWorldDeltaSeconds))
  (bind _plateforme_rot_z (Variables|Default|GetPlateforme%20rot-z))
  (bind _canon_rot_xy (Variables|Default|GetCanon%20rot-xy))
  (bind _rotation_speed (Variables|Default|GetRotation%20Speed))
  (bind _rotation_speed_2 (Variables|Default|GetRotation%20Speed))
  (bind _relativerotation (Variables|/Script/Engine.SceneComponent|GetRelativeRotation _plateforme_rot_z))
  (bind _relativerotation_2 (Variables|/Script/Engine.SceneComponent|GetRelativeRotation _canon_rot_xy))
  (bind _returnvalue_3 (Class|KismetMathLibrary|RInterptoConstant _relativerotation_2 "0, 0, 0" _returnvalue_2 _rotation_speed))
  (bind _returnvalue_4 (Class|KismetMathLibrary|RInterptoConstant _relativerotation "0, 0, 0" _returnvalue _rotation_speed_2))
  ;[1 1 1] Reset
  (Utilities|FlowControl|Gate true) ; enters at Close
)

(event Custom|Stop%20sweep
  (bind _newtrack_0 (Timeline|CameraSweep Stop)
    (:Update
      (CallFunction|ChangeState "NewEnumerator0")
      (Transformation|SetRelativeRotation (Variables|Default|GetCanon%20rot-xy) (Math|Rotator|MakeRotator 0.0 (Variables|Default|GetAngle%20Y) (Math|Float|Lerp 0.0 5e+01 _newtrack_0)) false false))))

(event Custom|Laser%20Off%20camera
  ;[1 1 1] Laser
  (bind _asbp_laser (Utilities|Casting|CastToBP_Laser (Variables|/Script/Engine.ChildActorComponent|GetChildActor (Variables|Default|Getlaser))))
  (bind _output_get (Variables|Default|SetAs%20BP%20Laser _asbp_laser))
  (Rendering|SetVisibility (Variables|/Game/_MAIN/BP/BP_Laser.BP_Laser_C|GetSM_Vision _output_get) false false)
  (Rendering|SetVisibility (Variables|/Game/_MAIN/BP/BP_Laser.BP_Laser_C|GetSM_Vision1 _output_get) false false)
  (Rendering|SetVisibility (Variables|/Game/_MAIN/BP/BP_Laser.BP_Laser_C|GetSM_Vision2 _output_get) false false))

(event Custom|Restart%20Sweep
  (CallFunction|ChangeState "NewEnumerator1")
  (Utilities|FlowControl|Sequence
    (:then_0
      (Utilities|FlowControl|DoOnce false
        (:Completed
          (Variables|Default|SetLastSeenRotation (Variables|/Script/Engine.SceneComponent|GetRelativeRotation (Variables|Default|GetCanon%20rot-xy)))
          (bind _newtrack_0 (Timeline|ReturnToSweep PlayFromStart)
            (:Update
              (Transformation|SetRelativeRotation (Variables|Default|GetCanon%20rot-xy) (Math|Rotator|Lerp(Rotator) (Variables|Default|GetLastSeenRotation) "0, 0, 0" _newtrack_0) false false)
              (CallFunction|ChangeState "NewEnumerator0")
              (bind _newtrack_0_2 (Timeline|CameraSweep PlayFromStart)
                (:Update
                  (CallFunction|ChangeState "NewEnumerator0")
                  (Transformation|SetRelativeRotation (Variables|Default|GetCanon%20rot-xy) (Math|Rotator|MakeRotator 0.0 (Variables|Default|GetAngle%20Y) (Math|Float|Lerp 0.0 5e+01 _newtrack_0_2)) false false))))))))
    (:then_1
      (Timeline|FollowTarget Stop
        (:Update
          (if (not (Variables|Default|GetStun))
            (Utilities|FlowControl|Sequence
              (:then_0
                (CallFunction|Lookat)
                (Utilities|FlowControl|DoOnce false :!label _label
                  (:Completed
                    (CallFunction|ChangeState "NewEnumerator1")
                    (Utilities|FlowControl|Delay 0.5)
                    (Utilities|IsValid (Variables|Default|GetTarget_Turret)
                      (:Is%20Valid
                        (Variables|Default|SetAttack%20Mode true))))))
              (:then_1
                (if (Variables|Default|GetAttack%20Mode)
                  (CallFunction|ChangeState "NewEnumerator2")
                  (Utilities|FlowControl|Delay (Variables|Default|GetVitesse%20de%20tir))
                  (Utilities|IsValid (Variables|Default|GetTarget_Turret)
                    (:Is%20Valid
                      (bind _outhit (Collision|LineTraceByChannel (Transformation|GetSocketLocation (Variables|Default|GetCanon%20rot-xy) "Pan") (Math|Vector|RotateVector (Transformation|GetActorLocation (Variables|Default|GetTarget_Turret)) (Math|Rotator|MakeRotator (Math|Random|RandomFloatinRange -2.0 2.0) 0.0 (Math|Random|RandomFloatinRange -2.0 2.0))) "TraceTypeQuery1" false (Utilities|Array|MakeArray self 0) "None"))
                      (Class|AISenseHearing|ReportNoiseEvent (.TraceEnd (Collision|BreakHitResult _outhit)) 1.0 (Variables|Default|GetPlayer) 0.0 "None"))))))))))
    (:then_2
      (Variables|Default|SetTarget_Turret 0))
    (:then_3
      (Variables|Default|SetAttack%20Mode false)
      (goto _label Reset))))

(event Custom|Laser%20on%20camera
  ;[1 1 1] Laser
  (bind _asbp_laser (Utilities|Casting|CastToBP_Laser (Variables|/Script/Engine.ChildActorComponent|GetChildActor (Variables|Default|Getlaser))))
  (bind _output_get (Variables|Default|SetAs%20BP%20Laser _asbp_laser))
  (Rendering|SetVisibility (Variables|/Game/_MAIN/BP/BP_Laser.BP_Laser_C|GetSM_Vision _output_get) true false)
  (Rendering|SetVisibility (Variables|/Game/_MAIN/BP/BP_Laser.BP_Laser_C|GetSM_Vision1 _output_get) true false)
  (Rendering|SetVisibility (Variables|/Game/_MAIN/BP/BP_Laser.BP_Laser_C|GetSM_Vision2 _output_get) true false))

(event Custom|Reset%20do%20once
  (Utilities|FlowControl|DoOnce false) ; enters at Reset
)

(event Custom|Stun%20cam
  (Variables|Default|SetStun true)
  (CallFunction|StopSweep)
  (CallFunction|StopFollowing)
  (CallFunction|StopReturntosweep)
  (Utilities|Time|ClearandInvalidateTimerbyHandle (Variables|Default|GetClear%20Timer)))

(event Custom|Stop%20returntosweep
  (bind _newtrack_0 (Timeline|ReturnToSweep Stop)
    (:Update
      (Transformation|SetRelativeRotation (Variables|Default|GetCanon%20rot-xy) (Math|Rotator|Lerp(Rotator) (Variables|Default|GetLastSeenRotation) "0, 0, 0" _newtrack_0) false false)
      (CallFunction|ChangeState "NewEnumerator0")
      (bind _newtrack_0_2 (Timeline|CameraSweep PlayFromStart)
        (:Update
          (CallFunction|ChangeState "NewEnumerator0")
          (Transformation|SetRelativeRotation (Variables|Default|GetCanon%20rot-xy) (Math|Rotator|MakeRotator 0.0 (Variables|Default|GetAngle%20Y) (Math|Float|Lerp 0.0 5e+01 _newtrack_0_2)) false false))))))

(event Custom|Unstun%20cam
  (Variables|Default|SetStun false)
  (CallFunction|RestartPatrol))

(event Custom|Restart%20patrol
  (Utilities|FlowControl|Sequence
    (:then_0
      (bind _asbp_first_person_character (Utilities|Casting|CastToBP_FirstPersonCharacter (Game|GetPlayerCharacter 0)))
      (Variables|Default|SetPlayer _asbp_first_person_character))
    (:then_1
      (bind _newtrack_0 (Timeline|CameraSweep Play)
        (:Update
          (CallFunction|ChangeState "NewEnumerator0")
          (Transformation|SetRelativeRotation (Variables|Default|GetCanon%20rot-xy) (Math|Rotator|MakeRotator 0.0 (Variables|Default|GetAngle%20Y) (Math|Float|Lerp 0.0 5e+01 _newtrack_0)) false false))))))

(event Custom|Select%20Target
  (bind _targetinrange (Variables|Default|GetTargetInRange))
  ;[1 1 1] Sélection de l'ennemi
  (if (Utilities|Array|IsValidIndex _targetinrange)
    (Variables|Default|SetTargetEnnemyDetected (Utilities|Array|Get(acopy) _targetinrange (Math|Random|RandomIntegerinRange 0 (Utilities|Array|LastIndex _targetinrange))))
    (CallFunction|BeginAim)
    (else
      (CallFunction|ResetAim))))

(event Custom|unshielded%20cam
  (Variables|Default|SetStun false))

(event Custom|shield%20cam
  (Variables|Default|SetStun true)
  (CallFunction|StopSweep)
  (CallFunction|StopFollowing)
  (CallFunction|StopReturntosweep)
  (CallFunction|RestartPatrol)
  (Utilities|Time|ClearandInvalidateTimerbyHandle (Variables|Default|GetClear%20Timer)))

(event Custom|BeginAim
  ;[1 1 1] Begin Aim
  (Utilities|FlowControl|Sequence
    (:then_0
      (goto _label Open))
    (:then_1
      (Utilities|FlowControl|Gate true :!label _label
        (:Exit
          (Utilities|IsValid (Variables|Default|GetTargetEnnemyDetected)
            (:Is%20Valid
              (Utilities|FlowControl|Sequence
                (:then_0
                  ;;[1 1 1] Tir
                  (Utilities|FlowControl|Delay (Variables|Default|GetVitesse%20de%20tir))
                  (Utilities|IsValid (Variables|Default|GetTargetEnnemyDetected)
                    (:Is%20Valid
                      (CallFunction|Shot self (Variables|Default|GetProjectile%20parent))
                      (Audio|PlaySound2D (Variables|Default|GetSound%20of%20Shot) 1.0 1.0 0.0 0 0))))
                (:then_1
                  (CallFunction|Lookat)
                  (Utilities|FlowControl|Delay (Utilities|Time|GetWorldDeltaSeconds))
                  (CallFunction|ContinueAim))))
            (:Is%20Not%20Valid
              (CallFunction|CancelAim)
              (CallFunction|ResetAim))))))))

(event Custom|ResetAim
  (bind _returnvalue (Utilities|Time|GetWorldDeltaSeconds))
  (bind _returnvalue_2 (Utilities|Time|GetWorldDeltaSeconds))
  (bind _plateforme_rot_z (Variables|Default|GetPlateforme%20rot-z))
  (bind _canon_rot_xy (Variables|Default|GetCanon%20rot-xy))
  (bind _rotation_speed (Variables|Default|GetRotation%20Speed))
  (bind _rotation_speed_2 (Variables|Default|GetRotation%20Speed))
  (bind _relativerotation (Variables|/Script/Engine.SceneComponent|GetRelativeRotation _plateforme_rot_z))
  (bind _relativerotation_2 (Variables|/Script/Engine.SceneComponent|GetRelativeRotation _canon_rot_xy))
  (bind _returnvalue_3 (Class|KismetMathLibrary|RInterptoConstant _relativerotation_2 "0, 0, 0" _returnvalue_2 _rotation_speed))
  (bind _returnvalue_4 (Class|KismetMathLibrary|RInterptoConstant _relativerotation "0, 0, 0" _returnvalue _rotation_speed_2))
  ;[1 1 1] Reset
  (Utilities|FlowControl|Sequence
    (:then_0
      (goto _label Open))
    (:then_1
      (Utilities|FlowControl|Gate true :!label _label
        (:Exit
          (Utilities|IsValid (Variables|Default|GetTargetEnnemyDetected)
            (:Is%20Valid
              (CallFunction|StopReset :!label _label_2))
            (:Is%20Not%20Valid
              (if (and (Math|Rotator|Equal(Rotator) _returnvalue_4 "0, 0, 0" 0.0001) (Math|Rotator|Equal(Rotator) _returnvalue_3 "0, 0, 0" 0.0001))
                (goto _label_2)
                (else
                  (Transformation|SetRelativeRotation (Variables|Default|GetPlateforme%20rot-z) _returnvalue_4 false false)
                  (Transformation|SetRelativeRotation (Variables|Default|GetCanon%20rot-xy) _returnvalue_3 false false)
                  (Utilities|FlowControl|Delay (Utilities|Time|GetWorldDeltaSeconds))
                  (CallFunction|ContinueReset))))))))))

(event Custom|Continue%20Aim
  (bind _targetinrange (Variables|Default|GetTargetInRange))
  ;[1 1 1] Begin Aim
  (Utilities|IsValid (Variables|Default|GetTargetEnnemyDetected)
    (:Is%20Valid
      (if (Variables|/Game/FirstPerson/Blueprints/BP_FirstPersonCharacter.BP_FirstPersonCharacter_C|GetHP%20Good? (Variables|Default|GetTargetEnnemyDetected))
        (Utilities|FlowControl|Gate true
          (:Exit
            (Utilities|IsValid (Variables|Default|GetTargetEnnemyDetected)
              (:Is%20Valid
                (Utilities|FlowControl|Sequence
                  (:then_0
                    ;;[1 1 1] Tir
                    (Utilities|FlowControl|Delay (Variables|Default|GetVitesse%20de%20tir))
                    (Utilities|IsValid (Variables|Default|GetTargetEnnemyDetected)
                      (:Is%20Valid
                        (CallFunction|Shot self (Variables|Default|GetProjectile%20parent))
                        (Audio|PlaySound2D (Variables|Default|GetSound%20of%20Shot) 1.0 1.0 0.0 0 0))))
                  (:then_1
                    (CallFunction|Lookat)
                    (Utilities|FlowControl|Delay (Utilities|Time|GetWorldDeltaSeconds))
                    (CallFunction|ContinueAim))))
              (:Is%20Not%20Valid
                (CallFunction|CancelAim :!label _label)
                (CallFunction|ResetAim)))))
        (else
          ;[1 1 1] Change de cible si HP no good
          (if (Utilities|Array|ContainsItem _targetinrange (Variables|Default|GetTargetEnnemyDetected))
            (Utilities|Array|RemoveItem _targetinrange (Variables|Default|GetTargetEnnemyDetected))
            (Variables|Default|SetTargetEnnemyDetected 0)
            (CallFunction|SelectTarget)))))
    (:Is%20Not%20Valid
      (goto _label))))

(event Custom|Begin
  (params (NewParam :type Actor%20Object%20Reference))
  ;[1 1 1] Détection de l'ennemi
  (bind _asbp_first_person_character (Utilities|Casting|CastToBP_FirstPersonCharacter (Game|GetPlayerCharacter 0)))
  (Utilities|Array|Add (Variables|Default|GetTargetInRange) _asbp_first_person_character)
  (Utilities|IsValid (Variables|Default|GetTargetEnnemyDetected)
    (:Is%20Not%20Valid
      (CallFunction|SelectTarget)
      ;[1 1 1] Gestion de l'emissive
      (Rendering|Material|SetScalarParameterValueonMaterials (Variables|Default|GetCanon%20rot-xy) "Emissive" 1.5e+02))))

(event Custom|Cancel%20Aim
  ;[1 1 1] Begin Aim
  (Utilities|FlowControl|Gate true) ; enters at Close
)

(event Custom|Stop%20following
  (Timeline|FollowTarget Stop
    (:Update
      (if (not (Variables|Default|GetStun))
        (Utilities|FlowControl|Sequence
          (:then_0
            (CallFunction|Lookat)
            (Utilities|FlowControl|DoOnce false
              (:Completed
                (CallFunction|ChangeState "NewEnumerator1")
                (Utilities|FlowControl|Delay 0.5)
                (Utilities|IsValid (Variables|Default|GetTarget_Turret)
                  (:Is%20Valid
                    (Variables|Default|SetAttack%20Mode true))))))
          (:then_1
            (if (Variables|Default|GetAttack%20Mode)
              (CallFunction|ChangeState "NewEnumerator2")
              (Utilities|FlowControl|Delay (Variables|Default|GetVitesse%20de%20tir))
              (Utilities|IsValid (Variables|Default|GetTarget_Turret)
                (:Is%20Valid
                  (bind _outhit (Collision|LineTraceByChannel (Transformation|GetSocketLocation (Variables|Default|GetCanon%20rot-xy) "Pan") (Math|Vector|RotateVector (Transformation|GetActorLocation (Variables|Default|GetTarget_Turret)) (Math|Rotator|MakeRotator (Math|Random|RandomFloatinRange -2.0 2.0) 0.0 (Math|Random|RandomFloatinRange -2.0 2.0))) "TraceTypeQuery1" false (Utilities|Array|MakeArray self 0) "None"))
                  (Class|AISenseHearing|ReportNoiseEvent (.TraceEnd (Collision|BreakHitResult _outhit)) 1.0 (Variables|Default|GetPlayer) 0.0 "None"))))))))))

(event Custom|Continue%20Reset
  (bind _returnvalue (Utilities|Time|GetWorldDeltaSeconds))
  (bind _returnvalue_2 (Utilities|Time|GetWorldDeltaSeconds))
  (bind _plateforme_rot_z (Variables|Default|GetPlateforme%20rot-z))
  (bind _canon_rot_xy (Variables|Default|GetCanon%20rot-xy))
  (bind _rotation_speed (Variables|Default|GetRotation%20Speed))
  (bind _rotation_speed_2 (Variables|Default|GetRotation%20Speed))
  (bind _relativerotation (Variables|/Script/Engine.SceneComponent|GetRelativeRotation _plateforme_rot_z))
  (bind _relativerotation_2 (Variables|/Script/Engine.SceneComponent|GetRelativeRotation _canon_rot_xy))
  (bind _returnvalue_3 (Class|KismetMathLibrary|RInterptoConstant _relativerotation_2 "0, 0, 0" _returnvalue_2 _rotation_speed))
  (bind _returnvalue_4 (Class|KismetMathLibrary|RInterptoConstant _relativerotation "0, 0, 0" _returnvalue _rotation_speed_2))
  ;[1 1 1] Reset
  (Utilities|FlowControl|Gate true
    (:Exit
      (Utilities|IsValid (Variables|Default|GetTargetEnnemyDetected)
        (:Is%20Valid
          (CallFunction|StopReset :!label _label))
        (:Is%20Not%20Valid
          (if (and (Math|Rotator|Equal(Rotator) _returnvalue_4 "0, 0, 0" 0.0001) (Math|Rotator|Equal(Rotator) _returnvalue_3 "0, 0, 0" 0.0001))
            (goto _label)
            (else
              (Transformation|SetRelativeRotation (Variables|Default|GetPlateforme%20rot-z) _returnvalue_4 false false)
              (Transformation|SetRelativeRotation (Variables|Default|GetCanon%20rot-xy) _returnvalue_3 false false)
              (Utilities|FlowControl|Delay (Utilities|Time|GetWorldDeltaSeconds))
              (CallFunction|ContinueReset))))))))

(event EventBeginPlay
  (if (not (Variables|Default|GetStun))
    (Utilities|FlowControl|Sequence
      (:then_0
        (bind _asbp_first_person_character (Utilities|Casting|CastToBP_FirstPersonCharacter (Game|GetPlayerCharacter 0)))
        (Variables|Default|SetPlayer _asbp_first_person_character))
      (:then_1
        (bind _newtrack_0 (Timeline|CameraSweep Play)
          (:Update
            (CallFunction|ChangeState "NewEnumerator0")
            (Transformation|SetRelativeRotation (Variables|Default|GetCanon%20rot-xy) (Math|Rotator|MakeRotator 0.0 (Variables|Default|GetAngle%20Y) (Math|Float|Lerp 0.0 5e+01 _newtrack_0)) false false)))))))

(event EventTick
  (params (DeltaSeconds :type Float%20%28single-precision%29))
  (bind _player (Variables|Default|GetPlayer))
  (bind _firstpersoncamera (Variables|/Game/FirstPerson/Blueprints/BP_FirstPersonCharacter.BP_FirstPersonCharacter_C|GetFirstPersonCamera _player))
  (bind _returnvalue (Transformation|GetWorldLocation _firstpersoncamera))
  (if (Variables|/Game/FirstPerson/Blueprints/BP_Rifle.BP_Rifle_C|GetPickedUp (Variables|/Game/FirstPerson/Blueprints/BP_FirstPersonCharacter.BP_FirstPersonCharacter_C|GetRifle (Variables|Default|GetPlayer)))
    (Utilities|FlowControl|Sequence
      (:then_0
        (Math|Float|CompareFloat (Transformation|GetDistanceTo (Game|GetPlayerCharacter 0)) (Variables|/Game/FirstPerson/Blueprints/BP_FirstPersonCharacter.BP_FirstPersonCharacter_C|GetInteraction%20Distance (Variables|Default|GetPlayer))
          (:>
            (Variables|Default|SetHighlight false))
          (:<
            (Variables|Default|SetHighlight true))))
      (:then_1
        (if (Variables|Default|GetHighlight)
          (if (Variables|/Game/FirstPerson/Blueprints/BP_FirstPersonCharacter.BP_FirstPersonCharacter_C|GetStunned (Variables|Default|GetPlayer))
            (Variables|/Script/Engine.PostProcessComponent|SetbEnabled (Variables|Default|GetPostProcess) false :!label _label)
            (Rendering|SetRenderCustomDepth (Variables|Default|GetCanon%20rot-xy) false)
            (else
              (bind _outhit (Collision|SphereTraceForObjects _returnvalue (+ _returnvalue (* (Math|Vector|GetForwardVector _firstpersoncamera) (Variables|/Game/FirstPerson/Blueprints/BP_FirstPersonCharacter.BP_FirstPersonCharacter_C|GetInteraction%20Distance (Variables|Default|GetPlayer)))) 2e+01 (Utilities|Array|MakeArray "ObjectTypeQuery3" "ObjectTypeQuery4") false (Utilities|Array|MakeArray (Variables|Default|GetPlayer)) "None" false))
              (if (.bBlockingHit (Collision|BreakHitResult _outhit))
                (bind _asbp_camera_brouilleur (Utilities|Casting|CastToBP_Camera_brouilleur (.HitActor (Collision|BreakHitResult _outhit)))
                  (:then
                    (switch Utilities|FlowControl|Switch|SwitchonBP_ToolGun_Mode (Variables|/Game/FirstPerson/Blueprints/BP_FirstPersonCharacter.BP_FirstPersonCharacter_C|GetSelection (Variables|Default|GetPlayer))
                      (:NewEnumerator0
                        (Variables|/Script/Engine.PostProcessComponent|SetbEnabled (Variables|Default|GetPostProcess) false :!label _label_2)
                        (Rendering|SetRenderCustomDepth (Variables|Default|GetPlateforme%20rot-z) false))
                      (:NewEnumerator1
                        (Variables|/Script/Engine.PostProcessComponent|SetbEnabled (Variables|Default|GetPostProcess) true)
                        (Rendering|SetRenderCustomDepth (Variables|BP_Camera_immune_C|GetCanon%20rot-xy _asbp_camera_brouilleur) true))))
                  (:CastFailed
                    (goto _label_2)))
                (else
                  (goto _label_2)))))
          (else
            (goto _label)))))))

(fn ConstructionScript)

(fn Shot
  (params (Projectile :type BP%20Projectile%20Parent%20Class%20Reference))
  (bind _returnvalue (Game|SpawnActorfromClass Projectile (Transformation|GetWorldTransform (Variables|Default|GetSpawn%20projectile)) "Undefined" 0 0))
  (Variables|Default|SetBullet _returnvalue))

(fn LineOfSight
  (bind _scene (Variables|Default|GetScene))
  (bind _returnvalue (Transformation|GetWorldLocation _scene))
  (for _index (range 0 (Variables|Default|GetNumTraces))
    (bind _outhit (Collision|LineTraceByChannel _returnvalue (+ (* (Math|Vector|RotateVector (Math|Vector|RotateVector (Math|Vector|GetForwardVector (Variables|Default|GetScene)) (Math|Rotator|MakeRotator 0.0 0.0 (/ (* (Variables|Default|GetNumTraces) (Variables|Default|GetDegreesperTrace)) -2.0))) (Math|Rotator|MakeRotator 0.0 0.0 (* _index (Variables|Default|GetDegreesperTrace)))) 1e+03) _returnvalue) "TraceTypeQuery1" false 0 "ForDuration"))
    (return _outhit)))

(fn Lookat
  (bind _canon_rot_xy (Variables|Default|GetCanon%20rot-xy))
  (bind _looktarget (Class|InterfaceInteract|GetLookTarget(Message) (Variables|Default|GetTarget_Turret)))
  (Transformation|SetWorldRotation _canon_rot_xy (Math|Rotator|FindLookatRotation (Transformation|GetWorldLocation _canon_rot_xy) _looktarget) false false))

(fn LookV2
  (params (Other%20Actor :type Actor%20Object%20Reference))
  (bind _canon_rot_xy (Variables|Default|GetCanon%20rot-xy))
  (bind _output_get (Variables|Default|SetOther%20Actor Other%20Actor))
  (bind _looktarget (Class|InterfaceInteract|GetLookTarget(Message) _output_get))
  (Transformation|SetWorldRotation _canon_rot_xy (Math|Rotator|FindLookatRotation (Transformation|GetWorldLocation _canon_rot_xy) _looktarget) false false))

(fn TestTrace
  (bind _outhit (Collision|SphereTraceByChannel (Transformation|GetWorldLocation (Variables|Default|GetScene)) (Transformation|GetActorLocation (Variables|Default|GetOther%20Actor)) 5.0 "TraceTypeQuery2" false 0 "None"))
  (return (.bBlockingHit (Collision|BreakHitResult _outhit)) _outhit))

(fn ChangeState
  (params (Selection :type AlertState%20Enum :default "NewEnumerator0"))
  (switch Utilities|FlowControl|Switch|SwitchonAlertState Selection
    (:NewEnumerator0
      (bind _asbp_laser (Utilities|Casting|CastToBP_Laser (Variables|/Script/Engine.ChildActorComponent|GetChildActor (Variables|Default|Getlaser))))
      (bind _output_get (Variables|Default|SetAs%20BP%20Laser _asbp_laser))
      (bind _output_get_2 (Variables|Default|SetLaser_Color "(R=0.132347,G=0.930287,B=1.000000,A=1.000000)"))
      (Rendering|Material|SetVectorParameterValueonMaterials (Variables|/Game/_MAIN/BP/BP_Laser.BP_Laser_C|GetSM_Vision _output_get) "Laser_Color" (Math|Conversions|ToVector(LinearColor) _output_get_2)))
    (:NewEnumerator1
      (bind _asbp_laser_2 (Utilities|Casting|CastToBP_Laser (Variables|/Script/Engine.ChildActorComponent|GetChildActor (Variables|Default|Getlaser))))
      (bind _output_get_3 (Variables|Default|SetAs%20BP%20Laser _asbp_laser_2))
      (bind _output_get_4 (Variables|Default|SetLaser_Color "(R=1.000000,G=0.891706,B=0.002064,A=1.000000)"))
      (Rendering|Material|SetVectorParameterValueonMaterials (Variables|/Game/_MAIN/BP/BP_Laser.BP_Laser_C|GetSM_Vision _output_get_3) "Laser_Color" (Math|Conversions|ToVector(LinearColor) _output_get_4)))
    (:NewEnumerator2
      (bind _asbp_laser_3 (Utilities|Casting|CastToBP_Laser (Variables|/Script/Engine.ChildActorComponent|GetChildActor (Variables|Default|Getlaser))))
      (bind _output_get_5 (Variables|Default|SetAs%20BP%20Laser _asbp_laser_3))
      (bind _output_get_6 (Variables|Default|SetLaser_Color "(R=0.942708,G=0.000000,B=0.018558,A=1.000000)"))
      (Rendering|Material|SetVectorParameterValueonMaterials (Variables|/Game/_MAIN/BP/BP_Laser.BP_Laser_C|GetSM_Vision _output_get_5) "Laser_Color" (Math|Conversions|ToVector(LinearColor) _output_get_6)))))