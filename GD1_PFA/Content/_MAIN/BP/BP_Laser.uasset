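; BP_Laser is a laser actor that animates three SMVision meshes by rotating them in pitch.
; On BeginPlay it starts three timelines, each with its own play rate variable.
; Each timeline lerps one mesh's relative pitch from zero toward a different maximum angle, so the beams move independently.
; A node applying LaserColor to the meshes' Laser_Color material parameter exists but is unconnected, so it never runs.
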(event EventBeginPlay
  (Utilities|FlowControl|Sequence
    (:then_0
      (Components|Timeline|SetPlayRate (Variables|Default|GetLaser%201) (Variables|Default|GetPlay%20Rate%201))
      (bind _newtrack_0 (Timeline|Laser%201 Play)
        (:Update
          (Transformation|SetRelativeRotation (Variables|Default|GetSM_Vision) (Math|Rotator|MakeRotator 0.0 (Math|Float|Lerp 0.0 2.0 _newtrack_0) 0.0) false false))))
    (:then_1
      (Components|Timeline|SetPlayRate (Variables|Default|GetLaser%202) (Variables|Default|GetPlay%20Rate%202))
      (bind _newtrack_0_2 (Timeline|Laser%202 Play)
        (:Update
          (Transformation|SetRelativeRotation (Variables|Default|GetSM_Vision1) (Math|Rotator|MakeRotator 0.0 (Math|Float|Lerp 0.0 5.0 _newtrack_0_2) 0.0) false false))))
    (:then_2
      (Components|Timeline|SetPlayRate (Variables|Default|GetLaser%203) (Variables|Default|GetPlay%20Rate%203))
      (bind _newtrack_0_3 (Timeline|Laser%203 Play)
        (:Update
          (Transformation|SetRelativeRotation (Variables|Default|GetSM_Vision2) (Math|Rotator|MakeRotator 0.0 (Math|Float|Lerp 0.0 1e+01 _newtrack_0_3) 0.0) false false))))))

(fn ConstructionScript)