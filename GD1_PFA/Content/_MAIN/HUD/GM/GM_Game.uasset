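; GM_Game is a game mode that tracks player damage and handles death.
; On BeginPlay it caches the GI_Main game instance and the BP_FirstPersonCharacter player.
; PertePV adds incoming damage to a running total, then calls Mort to compare it with the death threshold.
; On death, Mort rotates the first-person camera, disables movement and, after a short delay, opens the 2map_test level.
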(event Custom|Perte%20PV
  (params (Montant%20dégâts :type Integer))
  ;[1 1 1] Système de PV
  (Variables|Default|SetDégâts%20subis (+ Montant%20dégâts (Variables|Default|GetDégâts%20subis)))
  (CallFunction|Mort))

(event Custom|Mort
  (bind _joueur (Variables|Default|GetJoueur))
  ;[1 1 1] Système de PV
  (if (>= (Variables|Default|GetDégâts%20subis) (Variables|Default|GetValeur%20de%20mort))
    ;[1 1 1] Gère l'état de mort
    (Transformation|SetRelativeRotation (Variables|/Game/FirstPerson/Blueprints/BP_FirstPersonCharacter.BP_FirstPersonCharacter_C|GetFirstPersonCamera _joueur) "0, 0,90.000000" false false)
    (Pawn|Components|CharacterMovement|DisableMovement (Variables|/Script/Engine.Character|GetCharacterMovement _joueur))
    (Utilities|FlowControl|Delay 0.5)
    (Game|OpenLevel(byObjectReference) "/Game/_MAIN/Maps/2-map_test.2-map_test")))

(event EventBeginPlay
  (Utilities|FlowControl|Sequence
    (:then_0
      ;[1 1 1] Ref Game Instance
      (bind _asgi_main (Utilities|Casting|CastToGI_Main (Game|GetGameInstance)))
      (Variables|Default|SetGI_Main _asgi_main))
    (:then_1
      (bind _asbp_first_person_character (Utilities|Casting|CastToBP_FirstPersonCharacter (Game|GetPlayerCharacter 0)))
      (Variables|Default|SetJoueur _asbp_first_person_character))))

(fn ConstructionScript)