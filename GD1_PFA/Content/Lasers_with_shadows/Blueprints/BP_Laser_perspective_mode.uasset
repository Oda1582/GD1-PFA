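; Laser beam actor whose perspective scene capture feeds an R16f depth map to a beam material with smoke, scanning and surface trail effects.
; Construction clamps gizmo-driven distance, FOV and scan angle, scales the geometry, and refreshes an editor preview.
; BeginPlay reads mode and pattern from DT_Lasers, then animates the beam's pitch.
; Dynamic lasers rotate a per-frame, one-pixel-high capture; static animated ones capture a taller map once and scan it in the shader.
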(event Custom|call_in_editor_update
  ;[1 1 1] Checking is Render Target are valid which preventing creation of Render Target every time when we move Laser or change any variables
  (Utilities|IsValid (Variables|Default|GetRender_target)
    (:Is%20Valid
      (Variables|/Script/Engine.SceneCaptureComponent2D|SetFOVAngle (Variables|Default|GetSceneCaptureComponent2D) (Variables|Default|GetBeam_angle))
      ;[1 1 1] Set created Render Target to be used by SceneCaptureComponent
      (Variables|/Script/Engine.SceneCaptureComponent2D|SetTextureTarget (Variables|Default|GetSceneCaptureComponent2D) (Variables|Default|GetRender_target))
      ;[1 1 1] Create Dynamic Material Instance and set correspond variable
      (bind _returnvalue (Rendering|Material|CreateDynamicMaterialInstance (Variables|Default|GetLaser_geometry) 0 "/Game/Lasers_with_shadows/Materials/M_Laser_perspective.M_Laser_perspective" "None" :!class /Script/Engine.PrimitiveComponent))
      (Variables|Default|SetLaser_material _returnvalue)
      ;[1 1 1] Assign Created Render Target to correspond texture parameter in shader
      (Rendering|Material|SetTextureParameterValue (Variables|Default|Getlaser_material) "depth_map" (Variables|Default|GetRender_target))
      ;[0.3 1 0.3] Basic settings
      (Rendering|Material|SetScalarParameterValue (Variables|Default|GetLaser_material) "beam_distance" (.x (Variables|Laser_settings|GetFOV_&_Distance)) :!class /Script/Engine.MaterialInstanceDynamic)
      (Rendering|Material|SetScalarParameterValue (Variables|Default|GetLaser_material) "sq" 1.0 :!class /Script/Engine.MaterialInstanceDynamic)
      (Rendering|Material|SetScalarParameterValue (Variables|Default|GetLaser_material) "beam_angle" (Variables|Default|GetBeam_angle) :!class /Script/Engine.MaterialInstanceDynamic)
      (Rendering|Material|SetScalarParameterValue (Variables|Default|GetLaser_material) "beam_distance_static" (.x (Variables|Laser_settings|GetFOV_&_Distance)) :!class /Script/Engine.MaterialInstanceDynamic)
      ;[0.3 1 0.3] Laser dissipation and inverse square fallof for intensity
      (Rendering|Material|SetScalarParameterValue (Variables|Default|GetLaser_material) "dissipation_intensity" (Variables|Laser_settings|Getlaser_dissipation_intensity) :!class /Script/Engine.MaterialInstanceDynamic)
      (Rendering|Material|SetScalarParameterValue (Variables|Default|GetLaser_material) "laser_start_brightness" (Variables|Laser_settings|Getlaser_start_brightness) :!class /Script/Engine.MaterialInstanceDynamic)
      ;[0.3 1 0.3] Smoke
      (Rendering|Material|SetScalarParameterValue (Variables|Default|GetLaser_material) "smoke_vorticity_tiling" (Variables|Laser_settings|Getsmoke_vorticity_tiling) :!class /Script/Engine.MaterialInstanceDynamic)
      (Rendering|Material|SetScalarParameterValue (Variables|Default|GetLaser_material) "smoke_vortisity" (Variables|Laser_settings|Getsmoke_vortisity) :!class /Script/Engine.MaterialInstanceDynamic)
      (Rendering|Material|SetScalarParameterValue (Variables|Default|GetLaser_material) "smoke_tiling" (Variables|Laser_settings|Getsmoke_tiling) :!class /Script/Engine.MaterialInstanceDynamic)
      (Rendering|Material|SetScalarParameterValue (Variables|Default|GetLaser_material) "Smoke_density" (Variables|Laser_settings|GetSmoke_density) :!class /Script/Engine.MaterialInstanceDynamic)
      (Rendering|Material|SetScalarParameterValue (Variables|Default|GetLaser_material) "smoke_flow_speed" (Variables|Laser_settings|Getsmoke_flow_speed) :!class /Script/Engine.MaterialInstanceDynamic)
      ;[0.3 1 0.3] Beam sides mask
      (Rendering|Material|SetScalarParameterValue (Variables|Default|GetLaser_material) "side_beam_width" (Variables|Laser_settings|Getside_beam_width) :!class /Script/Engine.MaterialInstanceDynamic)
      (Rendering|Material|SetScalarParameterValue (Variables|Default|GetLaser_material) "beam_angle" (Variables|Default|GetBeam_angle) :!class /Script/Engine.MaterialInstanceDynamic)
      (Rendering|Material|SetScalarParameterValue (Variables|Default|GetLaser_material) "side_beams_intensity" (Variables|Laser_settings|Getside_beams_intensity) :!class /Script/Engine.MaterialInstanceDynamic)
      ;[0.3 1 0.3] Scanning mask
      (Rendering|Material|SetScalarParameterValue (Variables|Default|GetLaser_material) "scan_beam_speed" (Variables|Laser_settings|Getscan_beam_speed) :!class /Script/Engine.MaterialInstanceDynamic)
      (Rendering|Material|SetScalarParameterValue (Variables|Default|GetLaser_material) "scan_beam_size" (Variables|Laser_settings|Getscan_beam_size) :!class /Script/Engine.MaterialInstanceDynamic)
      (Rendering|Material|SetScalarParameterValue (Variables|Default|GetLaser_material) "scan_beam_hardness" (Variables|Laser_settings|Getscan_beam_hardness) :!class /Script/Engine.MaterialInstanceDynamic)
      (Rendering|Material|SetScalarParameterValue (Variables|Default|GetLaser_material) "scan_visibility" (Variables|Laser_settings|Getscan_visibility) :!class /Script/Engine.MaterialInstanceDynamic)
      (Rendering|Material|SetScalarParameterValue (Variables|Default|GetLaser_material) "ping_pong_mode" (Math|Conversions|ToFloat(Boolean) (Variables|Laser_settings|Getping_pong_mode)) :!class /Script/Engine.MaterialInstanceDynamic)
      ;[0.3 1 0.3] Beam on surface
      (Rendering|Material|SetScalarParameterValue (Variables|Default|GetLaser_material) "laser_trail_width" (Variables|Laser_settings|Getlaser_trail_width) :!class /Script/Engine.MaterialInstanceDynamic)
      (Rendering|Material|SetScalarParameterValue (Variables|Default|GetLaser_material) "laser_trail_intensity" (Variables|Laser_settings|Getlaser_trail_intensity) :!class /Script/Engine.MaterialInstanceDynamic)
      ;[0.3 1 0.3] laser_visibility
      (Rendering|Material|SetScalarParameterValue (Variables|Default|GetLaser_material) "laser_visibility" (Variables|Laser_settings|Getlaser_visibility) :!class /Script/Engine.MaterialInstanceDynamic)
      ;[0.3 1 0.3] laser_color
      (Rendering|Material|SetVectorParameterValue (Variables|Default|GetLaser_material) "laser_color" (Variables|Laser_settings|Getlaser_color) :!class /Script/Engine.MaterialInstanceDynamic))
    (:Is%20Not%20Valid
      ;[1 1 1] Create Render Target for in editor use
      (bind _returnvalue_2 (Rendering|CreateRenderTarget2D 1024 1 "RTF_R16f"))
      (bind _output_get (Variables|Default|SetRender_target _returnvalue_2))
      (Variables|/Script/Engine.TextureRenderTarget2D|SetAddressX _output_get "TA_Clamp")
      (Variables|/Script/Engine.TextureRenderTarget2D|SetAddressY _output_get "TA_Clamp"))))

(event EventBeginPlay
  (bind _returnvalue (Math|Trig|GetPI))
  (bind _animation_speed (Variables|Laser_settings|Getanimation_speed))
  (bind _scan_angle (Variables|Default|Getscan_angle))
  (bind _fov___distance (Variables|Laser_settings|GetFOV_&_Distance))
  (bind _quality (Variables|Default|Getquality))
  (bind _scan_angle_2 (Variables|Default|Getscan_angle))
  (bind _returnvalue_2 (/ (.x _fov___distance) 2.0))
  (bind _returnvalue_3 (/ _scan_angle_2 3.6e+02))
  (bind _returnvalue_4 (* 2.0 _returnvalue))
  (bind _returnvalue_5 (* _returnvalue_4 _returnvalue_2))
  (bind _returnvalue_6 (* _returnvalue_5 _returnvalue_3))
  (bind _returnvalue_7 (/ _returnvalue_6 1e+02))
  (bind _returnvalue_8 (/ _animation_speed _returnvalue_7))
  (Utilities|FlowControl|Sequence
    (:then_0
      ;[1 1 1] Setting variables by Data Tables
      (bind _returnvalue_9 (Utilities|GetDataTableRow "/Game/Lasers_with_shadows/Data_tables/DT_Lasers.DT_Lasers" (Utilities|String|StringToName (Utilities|String|EnumtoString (Variables|Laser_settings|GetAnimation%20pattern))))
        (:then
          (bind _returnvalue_10 (Utilities|GetDataTableRow "/Game/Lasers_with_shadows/Data_tables/DT_Lasers.DT_Lasers" (Utilities|String|StringToName (Utilities|String|EnumtoString (Variables|Laser_settings|GetLaser%20mode))))
            (:then
              (Variables|Default|Setis_Dynamic (.bool_value (Utilities|Struct|BreakS_Lasers _returnvalue_10)))
              (Variables|Default|Setanimation_pattern (.int_value (Utilities|Struct|BreakS_Lasers _returnvalue_9))))))))
    (:then_1
      ;[1 1 1] Create and setting up Render Target for runtime. "Quality variable" normally shouldnt be changed. Default value - 3000
      (bind _returnvalue_11 (Rendering|CreateRenderTarget2D (Math|Float|Truncate (* _quality (/ (Math|Trig|Tan(Degrees) (/ (Variables|Default|GetBeam_angle) 2.0)) (- 2.0 (Math|Trig|Cos(Degrees) (/ (Variables|Default|GetBeam_angle) 2.0)))))) (Math|Float|Truncate (Math|Float|SelectFloat (Math|Float|SelectFloat 1.0 (* _quality (/ (Math|Trig|Tan(Degrees) (Variables|Default|Getscan_angle)) (- 2.0 (Math|Trig|Cos(Degrees) (Variables|Default|Getscan_angle))))) (Variables|Default|Getis_Dynamic)) 1.0 (Variables|Laser_settings|Getis_Animate))) "RTF_R16f"))
      (bind _output_get (Variables|Default|SetRender_target _returnvalue_11))
      (Variables|/Script/Engine.TextureRenderTarget2D|SetAddressX _output_get "TA_Clamp")
      (Variables|/Script/Engine.TextureRenderTarget2D|SetAddressY _output_get "TA_Clamp")
      ;[1 1 1] Setting SceneCaptureComponent to render once/every frame
      (Variables|/Script/Engine.SceneCaptureComponent|SetbCaptureEveryFrame (Variables|Default|GetSceneCaptureComponent2D) (Variables|Default|Getis_Dynamic))
      ;[1 1 1] Set created Render Target to be used by SceneCaptureComponent
      (Variables|/Script/Engine.SceneCaptureComponent2D|SetTextureTarget (Variables|Default|GetSceneCaptureComponent2D) (Variables|Default|GetRender_target))
      ;[1 1 1] Create Dynamic Material Instance and set correspond variable
      (bind _returnvalue_12 (Rendering|Material|CreateDynamicMaterialInstance (Variables|Default|GetLaser_geometry) 0 "/Game/Lasers_with_shadows/Materials/M_Laser_perspective.M_Laser_perspective" "None" :!class /Script/Engine.PrimitiveComponent))
      (Variables|Default|SetLaser_material _returnvalue_12)
      ;[1 1 1] Assign Created Render Target to correspond texture parameter in shader
      (Rendering|Material|SetTextureParameterValue (Variables|Default|Getlaser_material) "depth_map" (Variables|Default|GetRender_target))
      ;[0.3 1 0.3] Basic settings
      (Rendering|Material|SetScalarParameterValue (Variables|Default|GetLaser_material) "beam_distance" (.x (Variables|Laser_settings|GetFOV_&_Distance)) :!class /Script/Engine.MaterialInstanceDynamic)
      (Rendering|Material|SetScalarParameterValue (Variables|Default|GetLaser_material) "sq" 1.0 :!class /Script/Engine.MaterialInstanceDynamic)
      (Rendering|Material|SetScalarParameterValue (Variables|Default|GetLaser_material) "beam_angle" (Variables|Default|GetBeam_angle) :!class /Script/Engine.MaterialInstanceDynamic)
      (Rendering|Material|SetScalarParameterValue (Variables|Default|GetLaser_material) "beam_distance_static" (.x (Variables|Laser_settings|GetFOV_&_Distance)) :!class /Script/Engine.MaterialInstanceDynamic)
      ;[0.3 1 0.3] Laser dissipation and inverse square fallof for intensity
      (Rendering|Material|SetScalarParameterValue (Variables|Default|GetLaser_material) "dissipation_intensity" (Variables|Laser_settings|Getlaser_dissipation_intensity) :!class /Script/Engine.MaterialInstanceDynamic)
      (Rendering|Material|SetScalarParameterValue (Variables|Default|GetLaser_material) "laser_start_brightness" (Variables|Laser_settings|Getlaser_start_brightness) :!class /Script/Engine.MaterialInstanceDynamic)
      ;[0.3 1 0.3] Smoke
      (Rendering|Material|SetScalarParameterValue (Variables|Default|GetLaser_material) "smoke_vorticity_tiling" (Variables|Laser_settings|Getsmoke_vorticity_tiling) :!class /Script/Engine.MaterialInstanceDynamic)
      (Rendering|Material|SetScalarParameterValue (Variables|Default|GetLaser_material) "smoke_vortisity" (Variables|Laser_settings|Getsmoke_vortisity) :!class /Script/Engine.MaterialInstanceDynamic)
      (Rendering|Material|SetScalarParameterValue (Variables|Default|GetLaser_material) "smoke_tiling" (Variables|Laser_settings|Getsmoke_tiling) :!class /Script/Engine.MaterialInstanceDynamic)
      (Rendering|Material|SetScalarParameterValue (Variables|Default|GetLaser_material) "Smoke_density" (Variables|Laser_settings|GetSmoke_density) :!class /Script/Engine.MaterialInstanceDynamic)
      (Rendering|Material|SetScalarParameterValue (Variables|Default|GetLaser_material) "smoke_flow_speed" (Variables|Laser_settings|Getsmoke_flow_speed) :!class /Script/Engine.MaterialInstanceDynamic)
      ;[0.3 1 0.3] Beam sides mask
      (Rendering|Material|SetScalarParameterValue (Variables|Default|GetLaser_material) "side_beam_width" (Variables|Laser_settings|Getside_beam_width) :!class /Script/Engine.MaterialInstanceDynamic)
      (Rendering|Material|SetScalarParameterValue (Variables|Default|GetLaser_material) "beam_angle" (Variables|Default|GetBeam_angle) :!class /Script/Engine.MaterialInstanceDynamic)
      (Rendering|Material|SetScalarParameterValue (Variables|Default|GetLaser_material) "side_beams_intensity" (Variables|Laser_settings|Getside_beams_intensity) :!class /Script/Engine.MaterialInstanceDynamic)
      ;[0.3 1 0.3] Scanning mask
      (Rendering|Material|SetScalarParameterValue (Variables|Default|GetLaser_material) "scan_beam_speed" (Variables|Laser_settings|Getscan_beam_speed) :!class /Script/Engine.MaterialInstanceDynamic)
      (Rendering|Material|SetScalarParameterValue (Variables|Default|GetLaser_material) "scan_beam_size" (Variables|Laser_settings|Getscan_beam_size) :!class /Script/Engine.MaterialInstanceDynamic)
      (Rendering|Material|SetScalarParameterValue (Variables|Default|GetLaser_material) "scan_beam_hardness" (Variables|Laser_settings|Getscan_beam_hardness) :!class /Script/Engine.MaterialInstanceDynamic)
      (Rendering|Material|SetScalarParameterValue (Variables|Default|GetLaser_material) "scan_visibility" (Variables|Laser_settings|Getscan_visibility) :!class /Script/Engine.MaterialInstanceDynamic)
      (Rendering|Material|SetScalarParameterValue (Variables|Default|GetLaser_material) "ping_pong_mode" (Math|Conversions|ToFloat(Boolean) (Variables|Laser_settings|Getping_pong_mode)) :!class /Script/Engine.MaterialInstanceDynamic)
      ;[0.3 1 0.3] Beam on surface
      (Rendering|Material|SetScalarParameterValue (Variables|Default|GetLaser_material) "laser_trail_width" (Variables|Laser_settings|Getlaser_trail_width) :!class /Script/Engine.MaterialInstanceDynamic)
      (Rendering|Material|SetScalarParameterValue (Variables|Default|GetLaser_material) "laser_trail_intensity" (Variables|Laser_settings|Getlaser_trail_intensity) :!class /Script/Engine.MaterialInstanceDynamic)
      ;[0.3 1 0.3] laser_visibility
      (Rendering|Material|SetScalarParameterValue (Variables|Default|GetLaser_material) "laser_visibility" (Variables|Laser_settings|Getlaser_visibility) :!class /Script/Engine.MaterialInstanceDynamic)
      ;[0.3 1 0.3] laser_color
      (Rendering|Material|SetVectorParameterValue (Variables|Default|GetLaser_material) "laser_color" (Variables|Laser_settings|Getlaser_color) :!class /Script/Engine.MaterialInstanceDynamic))
    (:then_2
      ;[1 1 1] Setting everything for animation if is_Animate are true
      (if (Variables|Laser_settings|Getis_Animate)
        ;[1 1 1] Set animation speed
        (Components|Timeline|SetPlayRate (Variables|Default|GetLaser_animation) (Math|Float|SelectFloat (/ _returnvalue_8 2.0) _returnvalue_8 (== (Variables|Default|Getanimation_pattern) 2)))
        ;[1 1 1] Pick animation pattern from Data Tables and set Laser_rot for later use
        (switch int (Variables|Default|Getanimation_pattern)
          (:0
            (bind (_direction _forward _ping_pong) (Timeline|Laser_animation Play)
              (:Update
                (Variables|Default|Setlaser_rot (Math|Rotator|Lerp(Rotator) (Math|Rotator|MakeRotator 0.0 _scan_angle 0.0) (Math|Rotator|MakeRotator 0.0 (* _scan_angle -1.0) 0.0) (Utilities|Select :Index (Variables|Default|Getanimation_pattern) :Option%200 _forward :Option%201 _forward :Option%202 _ping_pong :Option%203 _forward)))
                ;[1 1 1] Set rotation for Laser_geometry
                (Transformation|SetRelativeRotation (Variables|Default|GetLaser_geometry) (Variables|Default|Getlaser_rot) false false)
                ;[1 1 1] Rotate SceneCaptureComponent if Laser are in dynamic mode
                (if (Variables|Default|Getis_Dynamic)
                  (Transformation|SetRelativeRotation (Variables|Default|GetRot) (Variables|Default|Getlaser_rot) false false)
                  (else
                    ;[0.3 1 0.3] Shader basic setting for animation
                    (Rendering|Material|SetScalarParameterValue (Variables|Default|GetLaser_material) "sq" (/ (- 2.0 (Math|Trig|Cos(Degrees) (.pitch (Variables|Default|Getlaser_rot)))) (- 2.0 (Math|Trig|Cos(Degrees) (Variables|Default|Getscan_angle)))) :!class /Script/Engine.MaterialInstanceDynamic)
                    (Rendering|Material|SetScalarParameterValue (Variables|Default|GetLaser_material) "scan" (+ (/ (/ (Math|Trig|Tan(Degrees) (* (.pitch (Variables|Default|Getlaser_rot)) -1.0)) (* (Math|Trig|Tan(Degrees) (Variables|Default|Getscan_angle)) (- 2.0 (Math|Trig|Cos(Degrees) (/ (Variables|Default|GetBeam_angle) 2.0))))) 2.0) 0.5) :!class /Script/Engine.MaterialInstanceDynamic)
                    (Rendering|Material|SetScalarParameterValue (Variables|Default|GetLaser_material) "beam_distance" (* (.x (Variables|Laser_settings|GetFOV_&_Distance)) (Math|Trig|Cos(Degrees) (.pitch (Variables|Default|Getlaser_rot)))) :!class /Script/Engine.MaterialInstanceDynamic))))))
          (:1
            (Timeline|Laser_animation Reverse))
          (:2
            (Timeline|Laser_animation Play))
          (:3
            (Timeline|Laser_animation Play)))))
    (:then_3
      ;[1 1 1] Calculate and setup FOV
      (if (not (Variables|Default|Getis_Dynamic))
        (if (Variables|Laser_settings|Getis_Animate)
          (Variables|/Script/Engine.SceneCaptureComponent2D|SetFOVAngle (Variables|Default|GetSceneCaptureComponent2D) (* (Class|KismetMathLibrary|DegAtan (* (Math|Trig|Tan(Degrees) (/ (Variables|Default|GetBeam_angle) 2.0)) (- 2.0 (Math|Trig|Cos(Degrees) (Variables|Default|Getscan_angle))))) 2.0)))))))

(fn ConstructionScript
  (bind _billboard (Variables|Default|GetBillboard))
  (bind _max_fov (Variables|Default|Getmax_fov))
  (bind _max_scan_angle (Variables|Default|Getmax_scan_angle))
  (bind _returnvalue (Math|Trig|Sin(Degrees) _max_scan_angle))
  (bind _returnvalue_2 (Transformation|GetWorldTransform _billboard))
  (bind (_location _rotation) (Math|Transform|BreakTransform _returnvalue_2))
  ;[1 1 1] Setting Laser geometry size and maximum FOV clamping
  (Variables|Default|SetBeam_angle (Math|Float|Clamp(Float) (* (Class|KismetMathLibrary|DegAtan2 (.y (Variables|Laser_settings|GetFOV_&_Distance)) (.x (Variables|Laser_settings|GetFOV_&_Distance))) 2.0) 0.0 _max_fov))
  (Transformation|SetWorldTransform (Variables|Default|GetLaser_geometry) (Math|Transform|MakeTransform _location _rotation (Math|Vector|MakeVector (/ (.x (Variables|Laser_settings|GetFOV_&_Distance)) 2e+02) (* (Math|Trig|Tan(Degrees) (/ (Math|Float|Clamp(Float) (* (Class|KismetMathLibrary|DegAtan2 (.y (Variables|Laser_settings|GetFOV_&_Distance)) (.x (Variables|Laser_settings|GetFOV_&_Distance))) 2.0) 0.0 _max_fov) 2.0)) (/ (.x (Variables|Laser_settings|GetFOV_&_Distance)) 2e+02)) 1.0)) false false)
  (Utilities|FlowControl|Sequence
    (:then_0
      ;[1 1 1] Keeping Fov_&_Distance variable 3D gizmo in place
      (Variables|Laser_settings|SetFOV_&_Distance (Math|Vector|MakeVector (.x (Variables|Laser_settings|GetFOV_&_Distance)) (.y (Variables|Laser_settings|GetFOV_&_Distance)) 0.0))
      (Variables|Laser_settings|SetFOV_&_Distance (Math|Vector|MakeVector (.x (Variables|Laser_settings|GetFOV_&_Distance)) (Math|Float|Clamp(Float) (.y (Variables|Laser_settings|GetFOV_&_Distance)) 0.0 (* (.x (Variables|Laser_settings|GetFOV_&_Distance)) (Math|Trig|Tan(Degrees) (/ _max_fov 2.0)))) (.z (Variables|Laser_settings|GetFOV_&_Distance))))
      (if (< (.x (Variables|Laser_settings|GetFOV_&_Distance)) 0.0)
        (Variables|Laser_settings|SetFOV_&_Distance (Math|Vector|MakeVector 0.0 (.y (Variables|Laser_settings|GetFOV_&_Distance)) (.z (Variables|Laser_settings|GetFOV_&_Distance))))
        (elif (< (.y (Variables|Laser_settings|GetFOV_&_Distance)) 0.0)
          (Variables|Laser_settings|SetFOV_&_Distance (Math|Vector|MakeVector (.x (Variables|Laser_settings|GetFOV_&_Distance)) 0.0 0.0)))))
    (:then_1
      ;[1 1 1] Set scanning_angle variable and keep 3D gizmo in place (gizmo will moves circular around Laser center with clamping at 50 degree)
      (Variables|Laser_settings|SetScanning_angle (Math|Vector|MakeVector (* (.x (Variables|Laser_settings|GetFOV_&_Distance)) (Math|Float|Clamp(Float) (Math|Trig|Cos(Degrees) (Class|KismetMathLibrary|DegAtan2 (.z (Variables|Laser_settings|GetScanning_angle)) (.x (Variables|Laser_settings|GetScanning_angle)))) (Math|Trig|Cos(Degrees) _max_scan_angle))) 0.0 (* (.x (Variables|Laser_settings|GetFOV_&_Distance)) (Math|Float|Clamp(Float) (Math|Trig|Sin(Degrees) (Class|KismetMathLibrary|DegAtan2 (.z (Variables|Laser_settings|GetScanning_angle)) (.x (Variables|Laser_settings|GetScanning_angle)))) (* _returnvalue -1.0) _returnvalue))))
      (Variables|Default|Setscan_angle (Math|Float|Absolute(Float) (Class|KismetMathLibrary|DegAtan2 (.z (Variables|Laser_settings|GetScanning_angle)) (.x (Variables|Laser_settings|GetScanning_angle))))))
    (:then_2
      ;[1 1 1] Call in editor update
      (CallFunction|CallinEditorUpdate))))