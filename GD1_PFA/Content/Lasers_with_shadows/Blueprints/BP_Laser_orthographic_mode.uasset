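; Orthographic laser actor that draws a smoky, optionally sweeping beam with shadows from a scene-capture depth map.
; Construction sizes the beam from LaserSize, creates the R16f render target and feeds it with all look settings into a dynamic material.
; At play, dynamic lasers capture one pixel row every frame, moving the capture when animated.
; Static animated lasers capture the whole sweep once and pass timeline progress to the shader as "scan".
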(event Custom|call_in_editor_update
  (Utilities|FlowControl|Sequence
    (:then_0
      ;[1 1 1] Checking is Render Target are valid which preventing creation of Render Target every time when we move Laser of change any variables
      (Utilities|IsValid (Variables|Default|GetRender_target)
        (:Is%20Valid
          ;[1 1 1] Set Render Target ortho width
          (Variables|/Script/Engine.SceneCaptureComponent2D|SetOrthoWidth (Variables|Default|GetSceneCaptureComponent2D) (.x (Variables|Lasersettings|GetLaser_size)))
          ;[1 1 1] Set created Render Target to be used by SceneCaptureComponent
          (Variables|/Script/Engine.SceneCaptureComponent2D|SetTextureTarget (Variables|Default|GetSceneCaptureComponent2D) (Variables|Default|GetRender_target))
          ;[1 1 1] Create Dynamic Material Instance and set correspond variable
          (bind _returnvalue (Rendering|Material|CreateDynamicMaterialInstance (Variables|Default|GetLaser_geometry) 0 "/Game/Lasers_with_shadows/Materials/M_Laser_orthographic.M_Laser_orthographic" "None" :!class /Script/Engine.PrimitiveComponent))
          (Variables|Default|Setlaser_material _returnvalue)
          ;[1 1 1] Assign Created Render Target to correspond texture parameter in shader
          (Rendering|Material|SetTextureParameterValue (Variables|Default|Getlaser_material) "depth_map" (Variables|Default|GetRender_target))
          ;[0.3 1 0.3] Basic settings
          (Rendering|Material|SetScalarParameterValue (Variables|Default|Getlaser_material) "beam_distance" (* (.z (Variables|Lasersettings|GetLaser_size)) -1.0) :!class /Script/Engine.MaterialInstanceDynamic)
          (Rendering|Material|SetScalarParameterValue (Variables|Default|Getlaser_material) "Laser_size_X" (.x (Variables|Lasersettings|GetLaser_size)) :!class /Script/Engine.MaterialInstanceDynamic)
          (Rendering|Material|SetScalarParameterValue (Variables|Default|Getlaser_material) "bias" (Variables|Lasersettings|Getbias) :!class /Script/Engine.MaterialInstanceDynamic)
          ;[0.3 1 0.3] Distance dissipation mask
          (Rendering|Material|SetScalarParameterValue (Variables|Default|Getlaser_material) "dissipation_intensity" (Variables|Lasersettings|Getlaser_dissipation_intensity) :!class /Script/Engine.MaterialInstanceDynamic)
          ;[0.3 1 0.3] Smoke
          (Rendering|Material|SetScalarParameterValue (Variables|Default|Getlaser_material) "smoke_vorticity_tiling" (Variables|Lasersettings|Getsmoke_vorticity_tiling) :!class /Script/Engine.MaterialInstanceDynamic)
          (Rendering|Material|SetScalarParameterValue (Variables|Default|Getlaser_material) "smoke_vortisity" (Variables|Lasersettings|Getsmoke_vortisity) :!class /Script/Engine.MaterialInstanceDynamic)
          (Rendering|Material|SetScalarParameterValue (Variables|Default|Getlaser_material) "smoke_tiling" (Variables|Lasersettings|Getsmoke_tiling) :!class /Script/Engine.MaterialInstanceDynamic)
          (Rendering|Material|SetScalarParameterValue (Variables|Default|Getlaser_material) "Smoke_density" (Variables|Lasersettings|GetSmoke_density) :!class /Script/Engine.MaterialInstanceDynamic)
          (Rendering|Material|SetScalarParameterValue (Variables|Default|Getlaser_material) "smoke_flow_speed" (Variables|Lasersettings|Getsmoke_flow_speed) :!class /Script/Engine.MaterialInstanceDynamic)
          ;[0.3 1 0.3] Beam sides mask
          (Rendering|Material|SetScalarParameterValue (Variables|Default|Getlaser_material) "side_beam_width" (Variables|Lasersettings|Getside_beam_width) :!class /Script/Engine.MaterialInstanceDynamic)
          (Rendering|Material|SetScalarParameterValue (Variables|Default|Getlaser_material) "side_beams_intensity" (Variables|Lasersettings|Getside_beams_intensity) :!class /Script/Engine.MaterialInstanceDynamic)
          ;[0.3 1 0.3] Scanning mask
          (Rendering|Material|SetScalarParameterValue (Variables|Default|Getlaser_material) "scan_beam_speed" (Variables|Lasersettings|Getscan_beam_speed) :!class /Script/Engine.MaterialInstanceDynamic)
          (Rendering|Material|SetScalarParameterValue (Variables|Default|Getlaser_material) "scan_beam_size" (Variables|Lasersettings|Getscan_beam_size) :!class /Script/Engine.MaterialInstanceDynamic)
          (Rendering|Material|SetScalarParameterValue (Variables|Default|Getlaser_material) "scan_beam_hardness" (Variables|Lasersettings|Getscan_beam_hardness) :!class /Script/Engine.MaterialInstanceDynamic)
          (Rendering|Material|SetScalarParameterValue (Variables|Default|Getlaser_material) "scan_visibility" (Variables|Lasersettings|Getscan_visibility) :!class /Script/Engine.MaterialInstanceDynamic)
          (Rendering|Material|SetScalarParameterValue (Variables|Default|Getlaser_material) "ping_pong_mode" (Math|Conversions|ToFloat(Boolean) (Variables|Lasersettings|Getping_pong_mode)) :!class /Script/Engine.MaterialInstanceDynamic)
          ;[0.3 1 0.3] Beam on surface
          (Rendering|Material|SetScalarParameterValue (Variables|Default|Getlaser_material) "laser_trail_width" (Variables|Lasersettings|Getlaser_trail_width) :!class /Script/Engine.MaterialInstanceDynamic)
          (Rendering|Material|SetScalarParameterValue (Variables|Default|Getlaser_material) "laser_trail_intensity" (Variables|Lasersettings|Getlaser_trail_intensity) :!class /Script/Engine.MaterialInstanceDynamic)
          ;[0.3 1 0.3] Beam on parallel surfaces occlusion.
          (Rendering|Material|SetScalarParameterValue (Variables|Default|Getlaser_material) "beam_on_surface_ignore" (Variables|Lasersettings|Getbeam_on_perpendicular_surface_ignore) :!class /Script/Engine.MaterialInstanceDynamic)
          ;[0.3 1 0.3] Laser start brightness
          (Rendering|Material|SetScalarParameterValue (Variables|Default|Getlaser_material) "laser_start_position" (Variables|Lasersettings|Getlaser_start_position) :!class /Script/Engine.MaterialInstanceDynamic)
          (Rendering|Material|SetScalarParameterValue (Variables|Default|Getlaser_material) "laser_start_brightness_hardness" (Variables|Lasersettings|Getlaser_start_brightness_hardness) :!class /Script/Engine.MaterialInstanceDynamic)
          (Rendering|Material|SetScalarParameterValue (Variables|Default|Getlaser_material) "laser_start_brightness" (Variables|Lasersettings|Getlaser_start_brightness) :!class /Script/Engine.MaterialInstanceDynamic)
          ;[0.3 1 0.3] laser_visibility
          (Rendering|Material|SetScalarParameterValue (Variables|Default|Getlaser_material) "laser_visibility" (Variables|Lasersettings|Getlaser_visibility) :!class /Script/Engine.MaterialInstanceDynamic)
          ;[0.3 1 0.3] laser_color
          (Rendering|Material|SetVectorParameterValue (Variables|Default|Getlaser_material) "laser_color" (Variables|Lasersettings|Getlaser_color) :!class /Script/Engine.MaterialInstanceDynamic))
        (:Is%20Not%20Valid
          ;[1 1 1] Create and setting up Render Target for in editor use
          (bind _returnvalue_2 (Rendering|CreateRenderTarget2D (Math|Float|Truncate (.x (Variables|Lasersettings|GetLaser_size))) 1 "RTF_R16f" :!label _label))
          (bind _output_get (Variables|Default|SetRender_target _returnvalue_2))
          (Variables|/Script/Engine.TextureRenderTarget2D|SetAddressX _output_get "TA_Clamp")
          (Variables|/Script/Engine.TextureRenderTarget2D|SetAddressY _output_get "TA_Clamp"))))
    (:then_2
      ;[1 1 1] Forsing Render Target to be re-created again if laser size becoming too big for calculating and draw proper shadows
      (if (not (Math|Vector|Equal(Vector) (Variables|Lasersettings|GetLaser_size) (Variables|Default|GetLaser_size_last_value) 1e+03))
        (Variables|Default|SetLaser_size_last_value (Variables|Lasersettings|GetLaser_size))
        (goto _label)))))

(event EventBeginPlay
  (bind _laser_size (Variables|Lasersettings|GetLaser_size))
  (bind _animation_speed (Variables|Lasersettings|Getanimation_speed))
  (bind _laser_size_2 (Variables|Lasersettings|GetLaser_size))
  (bind _laser_size_3 (Variables|Lasersettings|GetLaser_size))
  (bind _is_animate (Variables|Lasersettings|Getis_animate))
  (bind (_x _y) (Math|Vector|BreakVector _laser_size))
  (bind _returnvalue (/ (.y _laser_size_3) 1e+02))
  (bind _returnvalue_2 (Math|Float|SelectFloat _y 1.0 _is_animate))
  (bind _returnvalue_3 (/ _animation_speed _returnvalue))
  (bind _returnvalue_4 (Math|Float|Truncate _returnvalue_2))
  (Utilities|FlowControl|Sequence
    (:then_0
      ;[1 1 1] Setting variables by Data Tables
      (bind _returnvalue_5 (Utilities|GetDataTableRow "/Game/Lasers_with_shadows/Data_tables/DT_Lasers.DT_Lasers" (Utilities|String|StringToName (Utilities|String|EnumtoString (Variables|Lasersettings|GetAnimation%20pattern))))
        (:then
          (bind _returnvalue_6 (Utilities|GetDataTableRow "/Game/Lasers_with_shadows/Data_tables/DT_Lasers.DT_Lasers" (Utilities|String|StringToName (Utilities|String|EnumtoString (Variables|Lasersettings|GetLaser%20mode))))
            (:then
              (Variables|Default|Setis_Dynamic (.bool_value (Utilities|Struct|BreakS_Lasers _returnvalue_6)))
              (Variables|Default|Setanimation_pattern (.int_value (Utilities|Struct|BreakS_Lasers _returnvalue_5))))))))
    (:then_1
      ;[1 1 1] Create and setting up Render Target for runtime
      (bind _returnvalue_7 (Rendering|CreateRenderTarget2D (Math|Float|Truncate _x) (Math|Integer|SelectInt 1 (Math|Integer|SelectInt 1 _returnvalue_4 (== _returnvalue_4 0)) (Variables|Default|Getis_Dynamic)) "RTF_R16f"))
      (bind _output_get (Variables|Default|SetRender_target _returnvalue_7))
      (Variables|/Script/Engine.TextureRenderTarget2D|SetAddressX _output_get "TA_Clamp")
      (Variables|/Script/Engine.TextureRenderTarget2D|SetAddressY _output_get "TA_Clamp")
      ;[1 1 1] Setting SceneCaptureComponent to render once/every frame
      (Variables|/Script/Engine.SceneCaptureComponent|SetbCaptureEveryFrame (Variables|Default|GetSceneCaptureComponent2D) (Variables|Default|Getis_Dynamic))
      ;[1 1 1] Placing SceneCaptureComponent to desired location
      (Transformation|AddRelativeLocation (Variables|Default|GetRot) (Math|Vector|MakeVector 0.0 (/ (Math|Float|SelectFloat 0.0 (Math|Float|SelectFloat (.y (Variables|Lasersettings|GetLaser_size)) 0.0 (Variables|Lasersettings|Getis_animate)) (Variables|Default|Getis_Dynamic)) 2.0) 0.0) false false)
      ;[1 1 1] Set created Render Target to be used by SceneCaptureComponent
      (Variables|/Script/Engine.SceneCaptureComponent2D|SetTextureTarget (Variables|Default|GetSceneCaptureComponent2D) (Variables|Default|GetRender_target))
      ;[1 1 1] Create Dynamic Material Instance and set correspond variable
      (bind _returnvalue_8 (Rendering|Material|CreateDynamicMaterialInstance (Variables|Default|GetLaser_geometry) 0 "/Game/Lasers_with_shadows/Materials/M_Laser_orthographic.M_Laser_orthographic" "None" :!class /Script/Engine.PrimitiveComponent))
      (Variables|Default|Setlaser_material _returnvalue_8)
      ;[1 1 1] Assign Created Render Target to correspond texture parameter in shader
      (Rendering|Material|SetTextureParameterValue (Variables|Default|Getlaser_material) "depth_map" (Variables|Default|GetRender_target))
      ;[0.3 1 0.3] Basic settings
      (Rendering|Material|SetScalarParameterValue (Variables|Default|Getlaser_material) "beam_distance" (* (.z (Variables|Lasersettings|GetLaser_size)) -1.0) :!class /Script/Engine.MaterialInstanceDynamic)
      (Rendering|Material|SetScalarParameterValue (Variables|Default|Getlaser_material) "Laser_size_X" (.x (Variables|Lasersettings|GetLaser_size)) :!class /Script/Engine.MaterialInstanceDynamic)
      (Rendering|Material|SetScalarParameterValue (Variables|Default|Getlaser_material) "bias" (Variables|Lasersettings|Getbias) :!class /Script/Engine.MaterialInstanceDynamic)
      ;[0.3 1 0.3] Distance dissipation mask
      (Rendering|Material|SetScalarParameterValue (Variables|Default|Getlaser_material) "dissipation_intensity" (Variables|Lasersettings|Getlaser_dissipation_intensity) :!class /Script/Engine.MaterialInstanceDynamic)
      ;[0.3 1 0.3] Smoke
      (Rendering|Material|SetScalarParameterValue (Variables|Default|Getlaser_material) "smoke_vorticity_tiling" (Variables|Lasersettings|Getsmoke_vorticity_tiling) :!class /Script/Engine.MaterialInstanceDynamic)
      (Rendering|Material|SetScalarParameterValue (Variables|Default|Getlaser_material) "smoke_vortisity" (Variables|Lasersettings|Getsmoke_vortisity) :!class /Script/Engine.MaterialInstanceDynamic)
      (Rendering|Material|SetScalarParameterValue (Variables|Default|Getlaser_material) "smoke_tiling" (Variables|Lasersettings|Getsmoke_tiling) :!class /Script/Engine.MaterialInstanceDynamic)
      (Rendering|Material|SetScalarParameterValue (Variables|Default|Getlaser_material) "Smoke_density" (Variables|Lasersettings|GetSmoke_density) :!class /Script/Engine.MaterialInstanceDynamic)
      (Rendering|Material|SetScalarParameterValue (Variables|Default|Getlaser_material) "smoke_flow_speed" (Variables|Lasersettings|Getsmoke_flow_speed) :!class /Script/Engine.MaterialInstanceDynamic)
      ;[0.3 1 0.3] Beam sides mask
      (Rendering|Material|SetScalarParameterValue (Variables|Default|Getlaser_material) "side_beam_width" (Variables|Lasersettings|Getside_beam_width) :!class /Script/Engine.MaterialInstanceDynamic)
      (Rendering|Material|SetScalarParameterValue (Variables|Default|Getlaser_material) "side_beams_intensity" (Variables|Lasersettings|Getside_beams_intensity) :!class /Script/Engine.MaterialInstanceDynamic)
      ;[0.3 1 0.3] Scanning mask
      (Rendering|Material|SetScalarParameterValue (Variables|Default|Getlaser_material) "scan_beam_speed" (Variables|Lasersettings|Getscan_beam_speed) :!class /Script/Engine.MaterialInstanceDynamic)
      (Rendering|Material|SetScalarParameterValue (Variables|Default|Getlaser_material) "scan_beam_size" (Variables|Lasersettings|Getscan_beam_size) :!class /Script/Engine.MaterialInstanceDynamic)
      (Rendering|Material|SetScalarParameterValue (Variables|Default|Getlaser_material) "scan_beam_hardness" (Variables|Lasersettings|Getscan_beam_hardness) :!class /Script/Engine.MaterialInstanceDynamic)
      (Rendering|Material|SetScalarParameterValue (Variables|Default|Getlaser_material) "scan_visibility" (Variables|Lasersettings|Getscan_visibility) :!class /Script/Engine.MaterialInstanceDynamic)
      (Rendering|Material|SetScalarParameterValue (Variables|Default|Getlaser_material) "ping_pong_mode" (Math|Conversions|ToFloat(Boolean) (Variables|Lasersettings|Getping_pong_mode)) :!class /Script/Engine.MaterialInstanceDynamic)
      ;[0.3 1 0.3] Beam on surface
      (Rendering|Material|SetScalarParameterValue (Variables|Default|Getlaser_material) "laser_trail_width" (Variables|Lasersettings|Getlaser_trail_width) :!class /Script/Engine.MaterialInstanceDynamic)
      (Rendering|Material|SetScalarParameterValue (Variables|Default|Getlaser_material) "laser_trail_intensity" (Variables|Lasersettings|Getlaser_trail_intensity) :!class /Script/Engine.MaterialInstanceDynamic)
      ;[0.3 1 0.3] Beam on parallel surfaces occlusion.
      (Rendering|Material|SetScalarParameterValue (Variables|Default|Getlaser_material) "beam_on_surface_ignore" (Variables|Lasersettings|Getbeam_on_perpendicular_surface_ignore) :!class /Script/Engine.MaterialInstanceDynamic)
      ;[0.3 1 0.3] Laser start brightness
      (Rendering|Material|SetScalarParameterValue (Variables|Default|Getlaser_material) "laser_start_position" (Variables|Lasersettings|Getlaser_start_position) :!class /Script/Engine.MaterialInstanceDynamic)
      (Rendering|Material|SetScalarParameterValue (Variables|Default|Getlaser_material) "laser_start_brightness_hardness" (Variables|Lasersettings|Getlaser_start_brightness_hardness) :!class /Script/Engine.MaterialInstanceDynamic)
      (Rendering|Material|SetScalarParameterValue (Variables|Default|Getlaser_material) "laser_start_brightness" (Variables|Lasersettings|Getlaser_start_brightness) :!class /Script/Engine.MaterialInstanceDynamic)
      ;[0.3 1 0.3] laser_visibility
      (Rendering|Material|SetScalarParameterValue (Variables|Default|Getlaser_material) "laser_visibility" (Variables|Lasersettings|Getlaser_visibility) :!class /Script/Engine.MaterialInstanceDynamic)
      ;[0.3 1 0.3] laser_color
      (Rendering|Material|SetVectorParameterValue (Variables|Default|Getlaser_material) "laser_color" (Variables|Lasersettings|Getlaser_color) :!class /Script/Engine.MaterialInstanceDynamic))
    (:then_2
      ;[1 1 1] Setting everything for animation if is_Animate are true
      (if (Variables|Lasersettings|Getis_animate)
        ;[1 1 1] Set animation speed
        (Components|Timeline|SetPlayRate (Variables|Default|GetLaser_animation) (Utilities|Select :Index (Variables|Default|Getanimation_pattern) :Option%200 _returnvalue_3 :Option%201 _returnvalue_3 :Option%202 (/ _returnvalue_3 2.0)))
        ;[1 1 1] Pick animation pattern from Data Tables and set Laser_rot for later use
        (switch int (Variables|Default|Getanimation_pattern)
          (:0
            (bind (_direction _forward _ping_pong) (Timeline|Laser_animation Play)
              (:Update
                (Transformation|SetRelativeLocation (Variables|Default|GetLaser_geometry) (Math|Vector|Lerp(Vector) (Math|Vector|MakeVector 0.0 0.0 0.0) (Math|Vector|MakeVector 0.0 (.y _laser_size_2) 0.0) (Utilities|Select :Index (Variables|Default|Getanimation_pattern) :Option%200 _forward :Option%201 _forward :Option%202 _ping_pong)) false false)
                ;[1 1 1] Animate SceneCaptureComponent if Laser are in dynamic mode
                (if (Variables|Default|Getis_Dynamic)
                  (Transformation|SetRelativeLocation (Variables|Default|GetRot) (Math|Vector|MakeVector (/ (.x _laser_size_2) 2.0) (.Y (Math|Vector|BreakVector (Math|Vector|Lerp(Vector) (Math|Vector|MakeVector 0.0 0.0 0.0) (Math|Vector|MakeVector 0.0 (.y _laser_size_2) 0.0) (Utilities|Select :Index (Variables|Default|Getanimation_pattern) :Option%200 _forward :Option%201 _forward :Option%202 _ping_pong)))) (/ (Variables|Lasersettings|Getbias) 2.0)) false false)
                  (else
                    ;[0.3 1 0.3] Shader setting for animation
                    (Rendering|Material|SetScalarParameterValue (Variables|Default|Getlaser_material) "scan" (Utilities|Select :Index (Variables|Default|Getanimation_pattern) :Option%200 _forward :Option%201 _forward :Option%202 _ping_pong) :!class /Script/Engine.MaterialInstanceDynamic))))))
          (:1
            (Timeline|Laser_animation Reverse))
          (:2
            (Timeline|Laser_animation Play)))))))

(fn ConstructionScript
  (bind _laser_geometry (Variables|Default|GetLaser_geometry))
  (Utilities|FlowControl|Sequence
    (:then_0
      ;[1 1 1] Keeping Laser_size variable 3D gizmo in place
      (if (< (.x (Variables|Lasersettings|GetLaser_size)) 0.0)
        (Variables|Lasersettings|SetLaser_size (Math|Vector|MakeVector 0.0 (.y (Variables|Lasersettings|GetLaser_size)) (.z (Variables|Lasersettings|GetLaser_size))))
        (elif (< (.y (Variables|Lasersettings|GetLaser_size)) 0.0)
          (Variables|Lasersettings|SetLaser_size (Math|Vector|MakeVector (.x (Variables|Lasersettings|GetLaser_size)) 0.0 (.z (Variables|Lasersettings|GetLaser_size))))
          (elif (> (.z (Variables|Lasersettings|GetLaser_size)) 0.0)
            (Variables|Lasersettings|SetLaser_size (Math|Vector|MakeVector (.x (Variables|Lasersettings|GetLaser_size)) (.y (Variables|Lasersettings|GetLaser_size)) 0.0))))))
    (:then_1
      (if true
        (Variables|Lasersettings|SetLaser_size (Math|Vector|MakeVector (.x (Variables|Lasersettings|GetLaser_size)) (Math|Float|SelectFloat (.y (Variables|Lasersettings|GetLaser_size)) 0.0 (Variables|Lasersettings|Getis_animate)) (.z (Variables|Lasersettings|GetLaser_size))))))
    (:then_2
      ;[1 1 1] Setting Laser geometry size and Rot with desired Bias
      (Transformation|SetWorldTransform (Variables|Default|GetLaser_geometry) (Math|Transform|MakeTransform (Transformation|GetWorldLocation _laser_geometry) (Transformation|GetWorldRotation _laser_geometry) (Math|Vector|MakeVector (/ (.X (Math|Vector|BreakVector (Variables|Lasersettings|GetLaser_size))) 2e+02) 1.0 (/ (Math|Float|Absolute(Float) (.Z (Math|Vector|BreakVector (Variables|Lasersettings|GetLaser_size)))) 2e+02))) false false)
      (Transformation|AddRelativeLocation (Variables|Default|GetRot) (Math|Vector|MakeVector (/ (.X (Math|Vector|BreakVector (Variables|Lasersettings|GetLaser_size))) 2.0) 0.0 (/ (Variables|Lasersettings|Getbias) 2.0)) false false))
    (:then_3
      ;[1 1 1] Call in editor update
      (CallFunction|CallinEditorUpdate))))