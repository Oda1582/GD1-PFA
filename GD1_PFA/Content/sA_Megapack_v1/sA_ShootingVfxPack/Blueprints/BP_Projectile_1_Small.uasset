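; Small projectile Blueprint from a shooting VFX pack that triggers impact effects and damage when its collision sphere hits something.
; BeginPlay assigns the configurable hit effect asset to the Hiteffects component.
; On hit, it activates that effect at the impact point, disables collision and spawns an impact actor.
; It then damages the first-person player character, regardless of what was hit, and destroys itself if that character cast succeeds.
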(event OnComponentBeginOverlap(Sphere1)
  (params (OverlappedComponent :type Primitive%20Component%20Object%20Reference) (OtherActor :type Actor%20Object%20Reference) (OtherComp :type Primitive%20Component%20Object%20Reference) (OtherBodyIndex :type Integer) (bFromSweep :type Boolean) (SweepResult :type Hit%20Result%20Structure%20%28by%20ref%29)))

(event OnComponentHit(Sphere1)
  (params (HitComponent :type Primitive%20Component%20Object%20Reference) (OtherActor :type Actor%20Object%20Reference) (OtherComp :type Primitive%20Component%20Object%20Reference) (NormalImpulse :type Vector :default "0, 0, 0") (Hit :type Hit%20Result%20Structure%20%28by%20ref%29))
  (bind _location (Collision|BreakHitResult Hit))
  (bind _hiteffects (Variables|Default|GetHiteffects))
  (Components|Activation|SetActive _hiteffects true false)
  (Transformation|SetWorldLocation _hiteffects _location false false)
  (Collision|SetCollisionEnabled (Variables|Default|GetSphere1) "NoCollision")
  (Game|SpawnActorfromClass (Variables|Default|GetImpactActor) (Math|Transform|MakeTransform _location) "Undefined" 0 0)
  (bind _asbp_first_person_character (Utilities|Casting|CastToBP_FirstPersonCharacter (Game|GetPlayerCharacter 0)))
  (Game|Damage|ApplyDamage _asbp_first_person_character 1e+01 0 0)
  (Actor|DestroyActor))

(event EventBeginPlay
  (Class|NiagaraComponent|SetAsset (Variables|Default|GetHiteffects) (Variables|Default|GetHitEffect) true))

(fn ConstructionScript)